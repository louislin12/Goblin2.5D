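; BP_Barrel is a destructible barrel that breaks and drops currency pickups when it takes damage.
; The first damage event crumbles the geometry collection cluster and spawns a few BP_Currency actors at scattered offsets, each with a random config from CoinConfigArray.
; A FadeDestroy timeline, started from the spawn loop, drives the material Opacity parameter and destroys the actor when finished.
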(event EventBeginPlay)

(event Collision|EventActorBeginOverlap
  (params (OtherActor :type Actor%20Object%20Reference)))

(event EventTick
  (params (DeltaSeconds :type Float%20%28single-precision%29)))

(event Game|Damage|EventAnyDamage
  (params (Damage :type Float%20%28single-precision%29) (DamageType :type Damage%20Type%20Object%20Reference) (InstigatedBy :type Controller%20Object%20Reference) (DamageCauser :type Actor%20Object%20Reference))
  (bind _returnvalue (Math|Random|RandomFloatinRange -5e+01 5e+01))
  (Utilities|FlowControl|DoOnce false
    (:Completed
      (Class|GeometryCollectionComponent|CrumbleCluster (Variables|Default|GetGC_SM_Barrel))
      (for _index (range 0 (Math|Random|RandomIntegerinRange 3 5))
        (Game|SpawnActorfromClass "/Game/Core/Blueprints/Currency/BP_Currency.BP_Currency_C" (Math|Transform|MakeTransform (+ (Transformation|GetActorLocation) (Math|Vector|MakeVector _returnvalue _returnvalue 5e+01)) "0, 0, 0" "1.000000,1.000000,1.000000") "AdjustIfPossibleButAlwaysSpawn" "MultiplyWithRoot" 0 (Utilities|ResolveSoftReference (.OutItem (Utilities|Array|Random (Variables|Default|GetCoinConfigArray)))) 0)
        (bind _newtrack_0 (Timeline|FadeDestroy Play)
          (:Update
            (Rendering|Material|SetScalarParameterValueonMaterials (Variables|Default|GetGC_SM_Barrel) "Opacity" _newtrack_0))
          (:Finished
            (Actor|DestroyActor)))))))

(fn ConstructionScript)