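; Player state Blueprint that connects the Mountea dialogue manager to the owning player's UI and input.
; When the dialogue widget changes on a local controller, it adds or removes it through the HUD as viewport manager, toggling input mode and mouse cursor.
; Manager state changes, gated by a cosmetic-events check, block look and move input while dialogue is active and release it when enabled or disabled.
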(event OnDialogueUserInterfaceChanged(MounteaDialogueManager)
  (params (DialogueWidgetClass :type User%20Widget%20Class%20Reference) (DialogueWidget :type User%20Widget%20Object%20Reference))
  (bind _returnvalue (Game|GetPlayerController))
  (Utilities|IsValid _returnvalue
    (:Is%20Valid
      (if (Pawn|IsLocalPlayerController _returnvalue)
        (Utilities|IsValid DialogueWidget
          (:Is%20Valid
            (Class|MounteaDialogueHUDStatics|AddChildWidgettoViewport (HUD|GetHUD (Game|GetPlayerController)) DialogueWidget (Utilities|Struct|MakeWidgetAdditionParams (Class|MounteaDialogueManagerStatics|GetDialogueWidgetZOrder (Variables|Default|GetMounteaDialogueManager)) "(Minimum=(X=0.000000,Y=0.000000),Maximum=(X=1.000000,Y=1.000000))" "(Left=0.000000,Top=0.000000,Right=0.000000,Bottom=0.000000)"))
            ;[1 1 1] This is optional and you might want to remove it in some cases.
            (Input|SetInputModeGameandUI (Game|GetPlayerController) (Class|MounteaDialogueManagerStatics|GetDialogueWidget (Variables|Default|GetMounteaDialogueManager)) "LockAlways" true false)
            (Variables|/Script/Engine.PlayerController|SetbShowMouseCursor (Game|GetPlayerController) true))
          (:Is%20Not%20Valid
            (Class|MounteaDialogueHUDStatics|RemoveChildWidgetfromViewport (HUD|GetHUD (Game|GetPlayerController)) (Class|MounteaDialogueManagerStatics|GetDialogueWidget (Variables|Default|GetMounteaDialogueManager)))
            (Input|SetInputModeGameOnly (Game|GetPlayerController) true)
            (Variables|/Script/Engine.PlayerController|SetbShowMouseCursor (Game|GetPlayerController) false)))))))

(event OnDialogueManagerStateChanged(MounteaDialogueManager)
  (params (NewState :type EDialogueManagerState%20Enum%20%28by%20ref%29 :default "EDMS_Disabled"))
  (bind _self self)
  (bind _returnvalue (Game|GetPlayerController _self))
  (Networking|CanExecuteCosmeticEvents
    (:True
      (switch Utilities|FlowControl|Switch|SwitchonEDialogueManagerState NewState
        (:EDMS_Disabled
          (Utilities|IsValid _returnvalue :!label _label
            (:Is%20Valid
              (Input|SetIgnoreLookInput _returnvalue false)
              (Input|SetIgnoreMoveInput _returnvalue false))))
        (:EDMS_Enabled
          (goto _label))
        (:EDMS_Active
          (Utilities|IsValid _returnvalue
            (:Is%20Valid
              (Input|SetIgnoreLookInput _returnvalue true)
              (Input|SetIgnoreMoveInput _returnvalue true))))))))

(fn ConstructionScript)