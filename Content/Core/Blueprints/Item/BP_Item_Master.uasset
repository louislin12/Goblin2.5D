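; BP_Item_Master is an item Blueprint, named as the master for items, that configures its BPCItem component from an ItemConfig asset.
; The Construction Script synchronously loads the soft-referenced config and copies its name, type and stackable flag into the component.
; Stack count and maximum are applied only for stackable items.
; The Event Graph holds no active logic.
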(event EventBeginPlay)

(event Collision|EventActorBeginOverlap
  (params (OtherActor :type Actor%20Object%20Reference)))

(event EventTick
  (params (DeltaSeconds :type Float%20%28single-precision%29)))

(fn ConstructionScript
  (bind _itemconfig (Variables|Default|GetItemConfig))
  (bind _output (Utilities|ResolveSoftReference _itemconfig))
  (bind _isstackable (Variables|/Script/Goblin25D.ItemConfigBase|GetIsStackable _output))
  (Utilities|LoadAssetBlocking _itemconfig)
  (Variables|/Script/AGR_Inventory_Runtime.AGR_ItemComponent|SetItemName (Variables|Default|GetBPC_Item) (Variables|/Script/Goblin25D.ItemConfigBase|GetName _output))
  (Variables|/Script/AGR_Inventory_Runtime.AGR_ItemComponent|SetItemType (Variables|Default|GetBPC_Item) (Variables|/Script/Goblin25D.ItemConfigBase|GetItemType _output))
  (Variables|/Script/AGR_Inventory_Runtime.AGR_ItemComponent|SetbIsStackable (Variables|Default|GetBPC_Item) _isstackable)
  (if _isstackable
    (Class|AGRItemComponent|SetStackCount (Variables|Default|GetBPC_Item) (Variables|/Script/Goblin25D.ItemConfigBase|GetStackCount _output))
    (Variables|/Script/AGR_Inventory_Runtime.AGR_ItemComponent|SetMaxStackCount (Variables|Default|GetBPC_Item) (Variables|/Script/Goblin25D.ItemConfigBase|GetMaxStackCount _output))))