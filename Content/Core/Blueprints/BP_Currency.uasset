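; BP_Currency is a flipbook pickup that grants coins or crystals to the character that overlaps it.
; The construction script sets the flipbook from a DT_Money row.
; On sphere overlap with a BPI_CharacterInterace actor, it plays a sound and runs a timeline that pulls the sprite toward player 0 while shrinking it.
; When finished, it adds the amount to the overlapped actor's inventory component and destroys itself.
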(event OnComponentBeginOverlap(Sphere)
  (params (OverlappedComponent :type Primitive%20Component%20Object%20Reference) (OtherActor :type Actor%20Object%20Reference) (OtherComp :type Primitive%20Component%20Object%20Reference) (OtherBodyIndex :type Integer) (bFromSweep :type Boolean) (SweepResult :type Hit%20Result%20Structure%20%28by%20ref%29))
  (bind _fb_money (Variables|Default|GetFB_Money))
  (if (Utilities|DoesObjectImplementInterface OtherActor "/Game/Core/Blueprints/Interfaces/BPI_CharacterInterace.BPI_CharacterInterace_C")
    (Variables|Default|SetOverlappedActor OtherActor)
    (Audio|PlaySound2D "/Game/Sound/Pickup_Cue.Pickup_Cue" 1.0 1.0 0.0 0 0)
    (bind _absorb_coin (Timeline|Timeline Play)
      (:Update
        (Transformation|SetWorldLocation _fb_money (Math|Vector|Lerp(Vector) (Transformation|GetWorldLocation (Variables|Default|GetFB_Money)) (Transformation|GetWorldLocation (Variables|/Script/Engine.Character|GetCapsuleComponent (Game|GetPlayerCharacter 0))) _absorb_coin) false false)
        (Transformation|SetRelativeScale3D _fb_money (Math|Vector|Lerp(Vector) "1.000000,1.000000,1.000000" "0, 0, 0" _absorb_coin)))
      (:Finished
        (CallFunction|AddCurrency)
        (Actor|DestroyActor)))))

(fn ConstructionScript
  (bind _returnvalue (Utilities|GetDataTableRow "/Game/DataTable/DT_Money.DT_Money" (.rowname (Variables|Default|GetMoneyType)))
    (:then
      (Sprite|SetFlipbook (Variables|Default|GetFB_Money) (.PaperFlipBook (Utilities|Struct|BreakS_Money _returnvalue))))))

(fn AddCurrency
  (bind _currencyamount (Variables|Default|GetCurrencyAmount))
  (bind _overlappedactor (Variables|Default|GetOverlappedActor))
  (bind _returnvalue (Class|AGRInventoryFunctionLibrary|GetInventoryComponent _overlappedactor))
  (Utilities|IsValid _returnvalue
    (:Is%20Valid
      (switch Utilities|FlowControl|Switch|SwitchonE_Currency (Variables|Default|GetCurrencyType)
        (:NewEnumerator2
          (Class|BPIInventory|InfluenceCrystalsAmount(Message) _returnvalue _currencyamount))
        (:NewEnumerator3
          (Class|BPIInventory|InfluenceCoinsAmount(Message) _returnvalue _currencyamount))))))