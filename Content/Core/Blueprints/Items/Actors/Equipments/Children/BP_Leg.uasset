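; BP_Leg is an equipment item Blueprint that toggles between equipped and unequipped when used, raising the wearer's max HP while worn.
; It responds to BPC_Item events, equipping non-visibly into the Chest slot despite its Leg name, with debug prints on each toggle.
; Equip and unequip synchronously load ItemConfig, then add or subtract its EffectValue through the inventory owner's stats component.
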(event OnItemEquipped(BPC_Item)
  (params (InventoryComponent :type AGR%20Inventory%20Component%20Object%20Reference) (EquipmentSlot :type Gameplay%20Tag%20Structure%20%28by%20ref%29))
  (bind _itemconfig (Variables|Default|GetItemConfig))
  (Utilities|LoadAssetBlocking _itemconfig)
  (bind _statscomponent (Class|BPICharacterInterace|GetStatsComponent(Message) (Components|GetOwner InventoryComponent)))
  (Default|AddValuetoMaxHP _statscomponent (Math|Conversions|ToFloat(Integer) (Variables|/Script/Goblin25D.ItemConfigBase|GetEffectValue (Utilities|ResolveSoftReference _itemconfig))) "NewEnumerator3"))

(event OnItemUnequipped(BPC_Item)
  (params (InventoryComponent :type AGR%20Inventory%20Component%20Object%20Reference) (EquipmentSlot :type Gameplay%20Tag%20Structure%20%28by%20ref%29))
  (bind _itemconfig (Variables|Default|GetItemConfig))
  (Utilities|LoadAssetBlocking _itemconfig)
  (bind _statscomponent (Class|BPICharacterInterace|GetStatsComponent(Message) (Components|GetOwner InventoryComponent)))
  (Default|AddValuetoMaxHP _statscomponent (* (Math|Conversions|ToFloat(Integer) (Variables|/Script/Goblin25D.ItemConfigBase|GetEffectValue (Utilities|ResolveSoftReference _itemconfig))) -1.0) "NewEnumerator3"))

(event OnItemUsed(BPC_Item)
  (params (InventoryComponent :type AGR%20Inventory%20Component%20Object%20Reference) (ActionType :type Gameplay%20Tag%20Structure%20%28by%20ref%29))
  (if (.ReturnValue (Class|AGRInventoryComponent|IsItemEquipped InventoryComponent self))
    (Class|AGRItemComponent|UnequipItem (Variables|Default|GetBPC_Item) InventoryComponent "(TagName=\"Player.Equipment.Slot.Chest\")")
    (Development|PrintString "UnEquipped")
    (else
      (Class|AGRItemComponent|EquipItem (Variables|Default|GetBPC_Item) InventoryComponent "(TagName=\"Player.Equipment.Slot.Chest\")" false)
      (Development|PrintString "Equipped"))))

(event EventBeginPlay
  (|CallParentFunction) ; This node is disabled and will not be called.\nDrag off pins to build functionality.
)

(event Collision|EventActorBeginOverlap
  (params (OtherActor :type Actor%20Object%20Reference))
  (|CallParentFunction OtherActor) ; This node is disabled and will not be called.\nDrag off pins to build functionality.
)

(event EventTick
  (params (DeltaSeconds :type Float%20%28single-precision%29))
  (|CallParentFunction DeltaSeconds) ; This node is disabled and will not be called.\nDrag off pins to build functionality.
)

(fn ConstructionScript
  (|CallParentFunction))