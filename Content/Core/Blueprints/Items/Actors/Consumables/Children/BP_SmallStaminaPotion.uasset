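; Small stamina potion item actor, a child consumable that restores stamina to its user.
; When its item component fires OnItemUsed, it blocking-loads the item config and gets the inventory owner's stats component through a message call.
; It increases stamina by the config's effect value, decrements the stack, and destroys the item once the stack is empty.
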(event OnItemUsed(BPC_Item)
  (params (InventoryComponent :type AGR%20Inventory%20Component%20Object%20Reference) (ActionType :type Gameplay%20Tag%20Structure%20%28by%20ref%29))
  (bind _itemconfig (Variables|Default|GetItemConfig))
  (bind _bpc_item (Variables|Default|GetBPC_Item))
  (Utilities|LoadAssetBlocking _itemconfig)
  (bind _statscomponent (Class|BPICharacterInterace|GetStatsComponent(Message) (Components|GetOwner InventoryComponent)))
  (Default|IncreaseStamina _statscomponent (Math|Conversions|ToFloat(Integer) (Variables|/Script/Goblin25D.ItemConfigBase|GetEffectValue (Utilities|ResolveSoftReference _itemconfig))))
  (Class|AGRItemComponent|SetStackCount _bpc_item (- (Class|AGRItemComponent|GetStackCount _bpc_item) 1))
  (if (< (Class|AGRItemComponent|GetStackCount _bpc_item) 1)
    (Class|AGRItemComponent|DestroyItem (Variables|Default|GetBPC_Item) InventoryComponent)))

(event EventBeginPlay
  (|CallParentFunction) ; This node is disabled and will not be called.\nDrag off pins to build functionality.
)

(event Collision|EventActorBeginOverlap
  (params (OtherActor :type Actor%20Object%20Reference))
  (|CallParentFunction OtherActor) ; This node is disabled and will not be called.\nDrag off pins to build functionality.
)

(event EventTick
  (params (DeltaSeconds :type Float%20%28single-precision%29))
  (|CallParentFunction DeltaSeconds) ; This node is disabled and will not be called.\nDrag off pins to build functionality.
)

(fn ConstructionScript
  (|CallParentFunction))