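; Blueprint function library of static quest helpers for starting quests, completing tasks and showing quest popups.
; Each call takes a player controller and forwards through its message getters to the quest component or player HUD.
; Task completion sends the given object's class as a string payload.
; A separate helper turns a payload string into a soft object reference, returning it only if valid.
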(fn CreateQuestPopup
  (params (PlayerController :type Player%20Controller%20Object%20Reference) (NotifyText :type Text) (QuestData :type Quest%20Data%20Soft%20Object%20Reference))
  (bind _hud (Class|BPICharacterInterace|GetPlayerHUD(Message) PlayerController))
  (Default|SetQuestPopup _hud NotifyText QuestData))

(fn PayloadtoSoftReference
  (params (Payload :type String))
  (bind _returnvalue (Utilities|MakeSoftObjectPath Payload))
  (bind _returnvalue_2 (Class|KismetSystemLibrary|ToSoftObjRef(SoftObjPath) _returnvalue))
  (if (Utilities|IsValidSoftObjectReference _returnvalue_2)
    (return _returnvalue_2)
    (else
      (return 0))))

(fn CompleteQuestTask
  (params (PlayerController :type Player%20Controller%20Object%20Reference) (TaskType :type E_TaskType%20Enum :default "NewEnumerator2") (ObjectToPayload :type Object%20Object%20Reference))
  (bind _questcomponent (Class|BPICharacterInterace|GetQuestComponent(Message) PlayerController))
  (Default|CompleteTask _questcomponent TaskType (Utilities|Array|MakeArray (Utilities|ToString(SoftClassReference) (Utilities|ResolveSoftReference (Utilities|GetClass ObjectToPayload))))))

(fn BeginQuest
  (params (PlayerController :type Player%20Controller%20Object%20Reference) (QuestData :type Quest%20Data%20Soft%20Object%20Reference))
  (bind _questcomponent (Class|BPICharacterInterace|GetQuestComponent(Message) PlayerController))
  (Default|BeginQuest _questcomponent PlayerController QuestData))