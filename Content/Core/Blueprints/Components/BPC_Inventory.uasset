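; Inventory component that tracks coin and crystal currencies along with slot capacity per item category.
; Influence events add an amount to a balance and broadcast the new total through a currency-change dispatcher.
; Max slots live in a map keyed by category, and free slots equal that limit minus the items returned by gameplay tag.
; Unknown categories yield zero, with the max-slot getter also printing a warning.
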(event EventBeginPlay)

(event EventTick
  (params (DeltaSeconds :type Float%20%28single-precision%29)))

(event EventInfluenceCoinsAmount
  (params (InfluenceAmount :type Integer))
  (bind _output_get (Variables|Default|SetCoinsAmount (+ InfluenceAmount (Variables|Default|GetCoinsAmount) 0)))
  (Default|CallOnCurrencyChanges "COIN" _output_get))

(event EventInfluenceCrystalsAmount
  (params (InfluenceAmount :type Integer))
  (bind _output_get (Variables|Default|SetCrystalsAmount (+ InfluenceAmount (Variables|Default|GetCrystalsAmount))))
  (Default|CallOnCurrencyChanges "CRYSTAL" _output_get))

(event EventSetInventoryMaxSlot
  (params (InventoryCategory :type Gameplay%20Tag%20Structure) (MaxSlot :type Integer))
  (Utilities|Map|Add (Variables|Default|GetCategoryMaxSlotsMap) InventoryCategory MaxSlot))

(fn GetAvailableSlots
  (params (ItemType :type Gameplay%20Tag%20Structure))
  (bind _categorymaxslotsmap (Variables|Default|GetCategoryMaxSlotsMap))
  (bind (_value _returnvalue) (Utilities|Map|Find _categorymaxslotsmap ItemType))
  (if _returnvalue
    (bind _returnvalue_2 (Class|AGRInventoryComponent|GetAllItemsbyGameplayTag ItemType))
    (return (- _value (Utilities|Array|Length _returnvalue_2)))
    (else
      (return 0))))

(fn GetInventoryMaxSlot
  (params (InventoryCategory :type Gameplay%20Tag%20Structure))
  (bind _categorymaxslotsmap (Variables|Default|GetCategoryMaxSlotsMap))
  (bind (_value _returnvalue) (Utilities|Map|Find _categorymaxslotsmap InventoryCategory))
  (if _returnvalue
    (return _value)
    (else
      (Development|PrintString (Utilities|String|ToString(Text) (Utilities|Text|FormatText "Inventory Category {1} Not Found" (GameplayTags|GetTagName InventoryCategory))))
      (return 0))))