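; Quest manager component that starts quests and tracks them as active, completed or failed, blocking active or completed ones from restarting.
; Each quest runs as a BP_QuestInstance whose completion and failure events update the lists and show popups, while CompleteTask broadcasts task events.
; Completion grants player 0 currency, EXP and loot through blocking soft-reference loads.
; The focused quest is broadcast on change and passes to the first active quest on completion, but not on failure.
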(event EventBeginPlay)

(event EventTick
  (params (DeltaSeconds :type Float%20%28single-precision%29)))

(fn BeginQuest
  (params (PlayerController :type Player%20Controller%20Object%20Reference) (QuestData :type Quest%20Data%20Soft%20Object%20Reference))
  (bind _questinstance (CallFunction|FindActiveQuestInstance QuestData))
  (Utilities|IsValid _questinstance
    (:Is%20Valid
      (Development|PrintString "Quest Already Active!"))
    (:Is%20Not%20Valid
      (if (Utilities|Array|ContainsItem (Variables|Default|GetAllCompletedQuests) QuestData)
        (Development|PrintString "Quest Already Completed!")
        (elif (Utilities|IsValidSoftObjectReference QuestData)
          (bind _returnvalue (Game|ConstructObjectfromClass "/Game/Core/Blueprints/Quests/BP_QuestInstance.BP_QuestInstance_C"))
          (Class|QuestInstance|ActivateQuest _returnvalue PlayerController QuestData)
          (Utilities|Array|Add (Variables|Default|GetAllActiveQuests) _returnvalue)
          (Utilities|Array|RemoveItem (Variables|Default|GetAllFailedQuests) QuestData)
          (EventDispatchers|BindEventtoOnQuestCompleted _returnvalue (EventDispatchers|CreateEvent :!event OnQuestCompleted))
          (EventDispatchers|BindEventtoOnQuestFailed _returnvalue (EventDispatchers|CreateEvent :!event OnQuestFailed))
          (CallFunction|CreateQuestPopup (Game|GetPlayerController 0) "New Quest" QuestData)
          (Utilities|IsValid (Variables|Default|GetActiveQuestInFocus)
            (:Is%20Not%20Valid
              (CallFunction|SetQuestinFocus _returnvalue)))
          (else
            (Development|PrintString "Quest Data is not valid!")))))))

(fn OnQuestCompleted
  (params (QuestInstance :type Quest%20Instance%20Object%20Reference) (QuestData :type Quest%20Data%20Soft%20Object%20Reference))
  (bind _allactivequests (Variables|Default|GetAllActiveQuests))
  (bind _output (Utilities|Array|Get(acopy) _allactivequests))
  (bind _asbp_quest_instance (Utilities|Casting|CastToBP_QuestInstance QuestInstance))
  (Utilities|Array|RemoveItem (Variables|Default|GetAllActiveQuests) _asbp_quest_instance)
  (Utilities|Array|Add (Variables|Default|GetAllCompletedQuests) QuestData)
  (EventDispatchers|UnbindallEventsfromOnQuestCompleted QuestInstance)
  (EventDispatchers|UnbindallEventsfromOnQuestFailed QuestInstance)
  (EventDispatchers|UnbindallEventsfromOnQuestStarted QuestInstance)
  (CallFunction|CreateQuestPopup (Game|GetPlayerController 0) "Quest Completed" QuestData)
  (CallFunction|GiveRewards QuestData)
  (if (== QuestInstance (Variables|Default|GetActiveQuestInFocus))
    (Utilities|IsValid _output
      (:Is%20Valid
        (CallFunction|SetQuestinFocus _output))
      (:Is%20Not%20Valid
        (CallFunction|SetQuestinFocus)))))

(fn OnQuestFailed
  (params (QuestInstance :type Quest%20Instance%20Object%20Reference) (QuestData :type Quest%20Data%20Soft%20Object%20Reference))
  (bind _asbp_quest_instance (Utilities|Casting|CastToBP_QuestInstance QuestInstance))
  (Utilities|Array|RemoveItem (Variables|Default|GetAllActiveQuests) _asbp_quest_instance)
  (Utilities|Array|Add (Variables|Default|GetAllFailedQuests) QuestData)
  (EventDispatchers|UnbindallEventsfromOnQuestCompleted QuestInstance)
  (EventDispatchers|UnbindallEventsfromOnQuestFailed QuestInstance)
  (EventDispatchers|UnbindallEventsfromOnQuestStarted QuestInstance)
  (CallFunction|CreateQuestPopup (Game|GetPlayerController 0) "Quest Failed" QuestData))

(fn FindActiveQuestInstance
  (params (QuestData :type Quest%20Data%20Soft%20Object%20Reference))
  (bind _array_element (Utilities|Array|ForEachLoopwithBreak (Variables|Default|GetAllActiveQuests) :!label _label)
    (:LoopBody
      (if (== (Variables|/Script/Goblin25D.QuestInstance|GetCurrentQuestData _array_element) QuestData)
        (LocalVariables|SetQuestInstanceL _array_element)
        (goto _label Break)))
    (:Completed
      (return (LocalVariables|GetQuestInstanceL)))))

(fn CompleteTask
  (params (TaskType :type E_TaskType%20Enum :default "NewEnumerator2") (Payload :type Array%20of%20Strings))
  (Default|CallOnTaskCompleted TaskType Payload))

(fn SetQuestinFocus
  (params (ActiveQuestInFocus :type BP%20Quest%20Instance%20Object%20Reference))
  (bind _output_get (Variables|Default|SetActiveQuestInFocus ActiveQuestInFocus))
  (Default|CallOnQuestSetinFocus _output_get))

(fn GiveRewards
  (params (QuestData :type Quest%20Data%20Soft%20Object%20Reference))
  (bind _returnvalue (Game|Player|GetPlayerPawn 0))
  (bind _output (Utilities|ResolveSoftReference QuestData))
  (bind _returnvalue_2 (Class|AGRInventoryFunctionLibrary|GetInventoryComponent _returnvalue))
  (Utilities|LoadAssetBlocking QuestData)
  (Class|BPIInventory|InfluenceCoinsAmount(Message) _returnvalue_2 (Variables|/Script/Goblin25D.QuestData|GetCoins _output))
  (Class|BPIInventory|InfluenceCrystalsAmount(Message) _returnvalue_2 (Variables|/Script/Goblin25D.QuestData|GetCrystals _output))
  (bind _statscomponent (Class|BPICharacterInterace|GetStatsComponent(Message) _returnvalue))
  (Default|GainEXP _statscomponent (Variables|/Script/Goblin25D.QuestData|GetExperience _output))
  (bind _returnvalue_3 (Class|QuestData|GetLoot _output))
  (for _array_element _returnvalue_3
    (Utilities|LoadAssetBlocking (.ItemReward (Utilities|Struct|BreakItemLoot _array_element)))
    (bind _returnvalue_4 (Utilities|LoadClassAssetBlocking (Variables|/Script/Goblin25D.ItemConfigBase|GetItemClass (Utilities|ResolveSoftReference (.ItemReward (Utilities|Struct|BreakItemLoot _array_element))))))
    (Class|AGRInventoryComponent|AddStacks (Class|AGRInventoryFunctionLibrary|GetInventoryComponent (Game|Player|GetPlayerPawn 0)) _returnvalue_4 (Class|KismetMathLibrary|ToInt64(Integer) (.Amount (Utilities|Struct|BreakItemLoot _array_element))))))