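; BP_QuestInstance runs a single quest for a player controller as a linear sequence of tasks.
; StartQuest blocking-loads the quest data, binds each task's started, completed and failed events, then activates the first task.
; Started tasks become CurrentTask and are broadcast through OnNewTaskActivated.
; Each completion activates the next task in the array or completes the quest after the last; task failure has an empty handler.
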(event EventStartQuest
  (params (InPlayerController :type Player%20Controller%20Object%20Reference) (InQuestData :type Quest%20Data%20Soft%20Object%20Reference%20%28by%20ref%29))
  (Variables|Default|SetPlayerController InPlayerController)
  (Utilities|LoadAssetBlocking InQuestData)
  (bind _output_get (Variables|Default|SetAllQuestTasks (Variables|/Script/Goblin25D.QuestData|GetQuestTasks (Utilities|ResolveSoftReference InQuestData))))
  (for _array_element _output_get
    (EventDispatchers|BindEventtoOnTaskStarted _array_element (EventDispatchers|CreateEvent :!event OnTaskStarted))
    (EventDispatchers|BindEventtoOnTaskCompleted _array_element (EventDispatchers|CreateEvent :!event OnTaskCompleted))
    (EventDispatchers|BindEventtoOnTaskFailed _array_element (EventDispatchers|CreateEvent :!event OnTaskFailed)))
  (Class|QuestTask|ActivateTask (Utilities|Array|Get(acopy) (Variables|Default|GetAllQuestTasks)) (Variables|Default|GetPlayerController)))

(fn OnTaskCompleted
  (params (Task :type Quest%20Task%20Object%20Reference))
  (bind _allquesttasks (Variables|Default|GetAllQuestTasks))
  (bind _returnvalue (Utilities|Array|FindItem _allquesttasks Task))
  (bind _returnvalue_2 (+ _returnvalue 1))
  (bind _output (Utilities|Array|Get(acopy) _allquesttasks _returnvalue_2))
  (Utilities|IsValid _output
    (:Is%20Valid
      (Class|QuestTask|ActivateTask _output (Variables|Default|GetPlayerController)))
    (:Is%20Not%20Valid
      (Class|QuestInstance|CompleteQuest))))

(fn OnTaskStarted
  (params (Task :type Quest%20Task%20Object%20Reference))
  (bind _output_get (Variables|Default|SetCurrentTask Task))
  (Default|CallOnNewTaskActivated _output_get))

(fn OnTaskFailed
  (params (Task :type Quest%20Task%20Object%20Reference)))