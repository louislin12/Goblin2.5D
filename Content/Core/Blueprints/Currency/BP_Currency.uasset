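; BP_Currency is a collectible coin or crystal pickup that adds currency to the inventory of the character that touches it.
; The construction script loads CoinConfig to set the currency type, amount and flipbook sprite.
; Sphere overlap plays a sound and a timeline that pulls the flipbook toward player 0 while shrinking it.
; When the timeline finishes, AddCurrency messages the overlapping actor's inventory component by type, then the pickup destroys itself.
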(event OnComponentBeginOverlap(Sphere)
  (params (OverlappedComponent :type Primitive%20Component%20Object%20Reference) (OtherActor :type Actor%20Object%20Reference) (OtherComp :type Primitive%20Component%20Object%20Reference) (OtherBodyIndex :type Integer) (bFromSweep :type Boolean) (SweepResult :type Hit%20Result%20Structure%20%28by%20ref%29))
  (bind _fb_money (Variables|Default|GetFB_Money))
  (if (Utilities|DoesObjectImplementInterface OtherActor "/Game/Core/Blueprints/Interfaces/BPI_CharacterInterace.BPI_CharacterInterace_C")
    (Variables|Default|SetOverlappedActor OtherActor)
    (Audio|PlaySound2D "/Game/Sound/Pickup_Cue.Pickup_Cue" 1.0 1.0 0.0 0 0)
    (bind _absorb_coin (Timeline|Timeline Play)
      (:Update
        (Transformation|SetWorldLocation _fb_money (Math|Vector|Lerp(Vector) (Transformation|GetWorldLocation (Variables|Default|GetFB_Money)) (Transformation|GetWorldLocation (Variables|/Script/Engine.Character|GetCapsuleComponent (Game|GetPlayerCharacter 0))) _absorb_coin) false false)
        (Transformation|SetRelativeScale3D _fb_money (Math|Vector|Lerp(Vector) "1.000000,1.000000,1.000000" "0, 0, 0" _absorb_coin)))
      (:Finished
        (CallFunction|AddCurrency)
        (Actor|DestroyActor)))))

(fn ConstructionScript
  (bind _coinconfig (Variables|Default|GetCoinConfig))
  (bind _output (Utilities|ResolveSoftReference _coinconfig))
  (bind _returnvalue (Utilities|LoadAssetBlocking _coinconfig))
  (Utilities|IsValid _returnvalue
    (:Is%20Valid
      (Variables|Default|SetCurrencyType (Variables|/Script/Goblin25D.CoinConfigBase|GetCurrencyType _output))
      (Variables|Default|SetCurrencyAmount (Variables|/Script/Goblin25D.CoinConfigBase|GetValue _output))
      (Sprite|SetFlipbook (Variables|Default|GetFB_Money) (Variables|/Script/Goblin25D.CoinConfigBase|GetFlipbook _output)))))

(fn AddCurrency
  (bind _currencyamount (Variables|Default|GetCurrencyAmount))
  (bind _overlappedactor (Variables|Default|GetOverlappedActor))
  (bind _returnvalue (Class|AGRInventoryFunctionLibrary|GetInventoryComponent _overlappedactor))
  (Utilities|IsValid _returnvalue
    (:Is%20Valid
      (switch Utilities|FlowControl|Switch|SwitchonECurrencyType (Variables|Default|GetCurrencyType)
        (:COIN
          (Class|BPIInventory|InfluenceCoinsAmount(Message) _returnvalue _currencyamount))
        (:CRYSTAL
          (Class|BPIInventory|InfluenceCrystalsAmount(Message) _returnvalue _currencyamount))))))