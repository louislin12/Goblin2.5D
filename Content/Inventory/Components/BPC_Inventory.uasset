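; BPC_Inventory is an inventory component that opens the inventory screen when the IA_Inventory input fires.
; On BeginPlay it creates and caches a WBP_Inventory widget and stores a BP_MainGoblin reference from the player character.
; The input event adds that widget to the viewport, shows the mouse cursor and switches to UI-only input focused on it.
; This graph has no closing logic and no item storage.
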(event Input|EnhancedActionEvents|EnhancedInputActionIA_Inventory
  (params (ActionValue :type Boolean) (ElapsedSeconds :type Float%20%28double-precision%29) (TriggeredSeconds :type Float%20%28double-precision%29) (InputAction :type Input%20Action%20Object%20Reference :default "/Game/Input/Actions/IA_Inventory.IA_Inventory"))
  (bind _returnvalue (Game|GetPlayerController 0))
  (UserInterface|Viewport|AddtoViewport (Variables|Default|GetInventoryWidget) 0)
  (Variables|/Script/Engine.PlayerController|SetbShowMouseCursor _returnvalue true)
  (Input|SetInputModeUIOnly _returnvalue (Variables|Default|GetInventoryWidget) "DoNotLock" false))

(event EventBeginPlay
  (bind _returnvalue (UserInterface|CreateWidget "/Game/Inventory/Widgets/WBP_Inventory.WBP_Inventory_C"))
  (Variables|Default|SetInventoryWidget _returnvalue)
  (bind _asbp_main_goblin (Utilities|Casting|CastToBP_MainGoblin (Game|GetPlayerCharacter 0)))
  (Variables|Default|SetMain%20Goblin%20Ref _asbp_main_goblin))