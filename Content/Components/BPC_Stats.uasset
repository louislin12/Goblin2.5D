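; Actor component that holds character stats: health, stamina, mana, experience and level, and damage.
; Stamina and mana functions write straight to HUD widgets through the player controller cached at BeginPlay, though mana changes use a zero amount.
; Health and damage functions raise change notifications instead, with damage split into base and equipment.
; Experience overflow triggers a level-up with effect, sound, level-scaled threshold and points.
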(event EventBeginPlay
  (bind _asbp_player_controller (Utilities|Casting|CastToBP_PlayerController (Game|GetPlayerController 0)))
  (Variables|Default|SetBP%20Player%20Controller _asbp_player_controller))

(fn IncreaseStamina
  (params (StaminaRecovered :type Float%20%28double-precision%29))
  (bind _bp_player_controller (Variables|Default|GetBP%20Player%20Controller))
  (bind _wbp_hud_overlay (Variables|/Game/Core/Blueprints/Character/BP_PlayerController.BP_PlayerController_C|GetWBP%20Hud%20Overlay _bp_player_controller))
  (bind _wbp_playestaminabar (Variables|/Game/Core/UI/Widgets/WBP_RPGHUD.WBP_RPGHUD_C|GetWBP_PlayeStaminaBar _wbp_hud_overlay))
  (if (not (>= (Variables|Default|GetCurrent%20Stamina) (Variables|Default|GetMaxHealth)))
    (Variables|Default|SetCurrent%20Stamina (Math|Float|Clamp(Float) (+ (Variables|Default|GetCurrent%20Stamina) StaminaRecovered) 0.0 (Variables|Default|GetMaxStamina)))
    (Variables|/Script/UMG.ProgressBar|SetPercent (Variables|/Game/Core/UI/Widgets/WBP_PlayeStaminaBar.WBP_PlayeStaminaBar_C|GetProgressBarStamina _wbp_playestaminabar) (Math|Float|SafeDivide (Variables|Default|GetCurrent%20Stamina) (Variables|Default|GetMaxStamina)))
    (Variables|/Script/UMG.TextBlock|SetText (Variables|/Game/Core/UI/Widgets/WBP_PlayeStaminaBar.WBP_PlayeStaminaBar_C|GetTextBlock_Stamina _wbp_playestaminabar) (Utilities|Text|ToText(Float) (Variables|Default|GetCurrent%20Stamina) "HalfToEven"))
    (Variables|/Script/UMG.TextBlock|SetText (Variables|/Game/Core/UI/Widgets/WBP_PlayeStaminaBar.WBP_PlayeStaminaBar_C|GetTextBlock_MaxStamina _wbp_playestaminabar) (Utilities|Text|ToText(Float) (Variables|Default|GetMaxStamina) "HalfToEven"))))

(fn DecreaseStamina
  (params (Staminaused :type Float%20%28double-precision%29))
  (bind _bp_player_controller (Variables|Default|GetBP%20Player%20Controller))
  (bind _wbp_hud_overlay (Variables|/Game/Core/Blueprints/Character/BP_PlayerController.BP_PlayerController_C|GetWBP%20Hud%20Overlay _bp_player_controller))
  (bind _wbp_playestaminabar (Variables|/Game/Core/UI/Widgets/WBP_RPGHUD.WBP_RPGHUD_C|GetWBP_PlayeStaminaBar _wbp_hud_overlay))
  (Variables|Default|SetCurrent%20Stamina (Math|Float|Clamp(Float) (- (Variables|Default|GetCurrent%20Stamina) Staminaused) 0.0 (Variables|Default|GetMaxStamina)))
  (Variables|/Script/UMG.ProgressBar|SetPercent (Variables|/Game/Core/UI/Widgets/WBP_PlayeStaminaBar.WBP_PlayeStaminaBar_C|GetProgressBarStamina _wbp_playestaminabar) (Math|Float|SafeDivide (Variables|Default|GetCurrent%20Stamina) (Variables|Default|GetMaxStamina)))
  (Variables|/Script/UMG.TextBlock|SetText (Variables|/Game/Core/UI/Widgets/WBP_PlayeStaminaBar.WBP_PlayeStaminaBar_C|GetTextBlock_Stamina _wbp_playestaminabar) (Utilities|Text|ToText(Float) (Variables|Default|GetCurrent%20Stamina) "HalfToEven"))
  (Variables|/Script/UMG.TextBlock|SetText (Variables|/Game/Core/UI/Widgets/WBP_PlayeStaminaBar.WBP_PlayeStaminaBar_C|GetTextBlock_MaxStamina _wbp_playestaminabar) (Utilities|Text|ToText(Float) (Variables|Default|GetMaxStamina) "HalfToEven"))
  (Variables|Default|SetNoStamina? (<= (Variables|Default|GetCurrent%20Stamina) 0.0))
  (return false))

(fn IncreaseMana
  (if (not (>= (Variables|Default|GetMana) (Variables|Default|GetMaxMana)))
    (Variables|Default|SetMaxMana (Math|Float|Clamp(Float) (+ (Variables|Default|GetMana) 0.0) 0.0 (Variables|Default|GetMaxMana)))
    (Variables|/Script/UMG.ProgressBar|SetPercent (Variables|/Game/Core/UI/Widgets/WBP_RPGHUD.WBP_RPGHUD_C|GetManaBar (Variables|/Game/Core/Blueprints/Character/BP_PlayerController.BP_PlayerController_C|GetWBP%20Hud%20Overlay (Variables|Default|GetBP%20Player%20Controller))) (/ (Variables|Default|GetMana) (Variables|Default|GetMaxMana)))))

(fn DecreaseMana
  (if (not (<= (Variables|Default|GetMana) 0.0))
    (Variables|Default|SetMana (Math|Float|Clamp(Float) (- (Variables|Default|GetMana) 0.0) 0.0 (Variables|Default|GetMaxMana)))
    (Variables|/Script/UMG.ProgressBar|SetPercent (Variables|/Game/Core/UI/Widgets/WBP_RPGHUD.WBP_RPGHUD_C|GetManaBar (Variables|/Game/Core/Blueprints/Character/BP_PlayerController.BP_PlayerController_C|GetWBP%20Hud%20Overlay (Variables|Default|GetBP%20Player%20Controller))) (/ (Variables|Default|GetMana) (Variables|Default|GetMaxMana)))))

(fn GainEXP
  (params (EXP%20Gained :type Integer))
  (if (>= (+ (Variables|Default|GetCurrentEXP) EXP%20Gained) (Variables|Default|GetLevelupEXPNeed))
    (Variables|Default|SetCurrentEXP (- (+ (Variables|Default|GetCurrentEXP) EXP%20Gained) (Variables|Default|GetLevelupEXPNeed)))
    (Effects|SpawnEmitterAttached "/Game/AdvancedMagicFX03/Particles/Update.Update" 0 "None" "0, 0, 0" "0, 0, 0" "1.000000,1.000000,1.000000" "SnapToTarget")
    (Audio|PlaySound2D "/Engine/VREditor/Sounds/UI/Camera_Shutter.Camera_Shutter" 1.0 1.0 0.0 0 0)
    (Math|Integer|IncrementInt (Variables|Default|GetLevel)
      (:%20%20
        (Variables|Default|SetLevelupEXPNeed (* (Variables|Default|GetLevel) 120))
        (Variables|Default|SetLevelupPoint (+ (Variables|Default|GetLevelupPoint) 3))
        (Variables|/Game/Core/UI/Widgets/WBP_EXP.WBP_EXP_C|SetPercent (Variables|/Game/Core/UI/Widgets/WBP_RPGHUD.WBP_RPGHUD_C|GetWBP_EXP (Variables|/Game/Core/Blueprints/Character/BP_PlayerController.BP_PlayerController_C|GetWBP%20Hud%20Overlay (Variables|Default|GetBP%20Player%20Controller))) (/ (Variables|Default|GetLevel) (Variables|Default|GetLevelupEXPNeed)))))
    (else
      (Variables|Default|SetCurrentEXP (+ (Variables|Default|GetCurrentEXP) EXP%20Gained)))))

(fn AddValuetoHealth
  (params (Value :type Float%20%28double-precision%29) (Instigator :type Actor%20Object%20Reference))
  (Variables|Default|SetCurrentHealth (Math|Float|Clamp(Float) (+ Value (Variables|Default|GetCurrentHealth)) 0.0 (Variables|Default|GetMaxHealth)))
  (Default|CallOnHealthChanged (Variables|Default|GetCurrentHealth) (Variables|Default|GetMaxHealth) Instigator))

(fn AddValuetoDamage
  (params (Value :type Float%20%28double-precision%29) (DamageStatType :type E_DamageStatType%20Enum :default "NewEnumerator2"))
  (switch Utilities|FlowControl|Switch|SwitchonE_DamageStatType DamageStatType
    (:NewEnumerator2
      (Variables|Default|SetBaseDamage (+ Value (Utilities|Select :Index DamageStatType :NewEnumerator2 (Variables|Default|GetBaseDamage) :NewEnumerator3 (Variables|Default|GetEquipmentDamage)))))
    (:NewEnumerator3
      (Variables|Default|SetEquipmentDamage (+ Value (Utilities|Select :Index DamageStatType :NewEnumerator2 (Variables|Default|GetBaseDamage) :NewEnumerator3 (Variables|Default|GetEquipmentDamage))))))
  (Default|CallOnDamageChanged (Variables|Default|GetBaseDamage) (Variables|Default|GetEquipmentDamage) (+ (Variables|Default|GetBaseDamage) (Variables|Default|GetEquipmentDamage))))

(fn SetBaseDamage
  (params (Value :type Float%20%28double-precision%29))
  (Variables|Default|SetBaseDamage (+ Value (Variables|Default|GetBaseDamage)))
  (Default|CallOnDamageChanged (Variables|Default|GetBaseDamage) (Variables|Default|GetEquipmentDamage) (+ (Variables|Default|GetBaseDamage) (Variables|Default|GetEquipmentDamage))))