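; RPG component that tracks clamped health and stamina and mirrors them on the player's HUD.
; BeginPlay caches BP_PlayerController from player 0, and each increase or decrease function writes directly to its HUD overlay's bars and text.
; DecreaseHealth returns whether health is depleted, while DecreaseStamina sets NoStamina but always returns false.
; IncreaseStamina gates recovery against MaxHealth rather than MaxStamina.
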(event EventBeginPlay
  (bind _asbp_player_controller (Utilities|Casting|CastToBP_PlayerController (Game|GetPlayerController 0)))
  (Variables|Default|SetBP%20Player%20Controller _asbp_player_controller))

(fn DecreaseHealth
  (params (IncomingDamage :type Float%20%28double-precision%29))
  (bind _bp_player_controller (Variables|Default|GetBP%20Player%20Controller))
  (bind _wbp_hud_overlay (Variables|/Game/Bluepints/BP_PlayerController.BP_PlayerController_C|GetWBP%20Hud%20Overlay _bp_player_controller))
  (bind _wbp_playerhealthbar (Variables|/Game/Widgets/WBP_RPGHUD.WBP_RPGHUD_C|GetWBP_PlayerHealthBar _wbp_hud_overlay))
  (Variables|Default|SetCurrentHealth (Math|Float|Clamp(Float) (- (Variables|Default|GetCurrentHealth) IncomingDamage) 0.0 (Variables|Default|GetMaxHealth)))
  (Variables|/Script/UMG.ProgressBar|SetPercent (Variables|/Game/Widgets/WBP_PlayerHealthBar.WBP_PlayerHealthBar_C|GetProgressBarHealth _wbp_playerhealthbar) (Math|Float|SafeDivide (Variables|Default|GetCurrentHealth) (Variables|Default|GetMaxHealth)))
  (Variables|/Script/UMG.TextBlock|SetText (Variables|/Game/Widgets/WBP_PlayerHealthBar.WBP_PlayerHealthBar_C|GetTextBlock_Health _wbp_playerhealthbar) (Utilities|Text|ToText(Float) (Variables|Default|GetCurrentHealth) "HalfToEven"))
  (Variables|/Script/UMG.TextBlock|SetText (Variables|/Game/Widgets/WBP_PlayerHealthBar.WBP_PlayerHealthBar_C|GetTextBlock_MaxHealth _wbp_playerhealthbar) (Utilities|Text|ToText(Float) (Variables|Default|GetMaxHealth) "HalfToEven"))
  (bind _output_get (Variables|Default|SetIsDefeated? (<= (Variables|Default|GetCurrentHealth) 0.0)))
  (return _output_get))

(fn IncreaseHealth
  (params (IncomingHeal :type Float%20%28double-precision%29))
  (bind _bp_player_controller (Variables|Default|GetBP%20Player%20Controller))
  (bind _wbp_hud_overlay (Variables|/Game/Bluepints/BP_PlayerController.BP_PlayerController_C|GetWBP%20Hud%20Overlay _bp_player_controller))
  (bind _wbp_playerhealthbar (Variables|/Game/Widgets/WBP_RPGHUD.WBP_RPGHUD_C|GetWBP_PlayerHealthBar _wbp_hud_overlay))
  (if (not (>= (Variables|Default|GetCurrentHealth) (Variables|Default|GetMaxHealth)))
    (Variables|Default|SetCurrentHealth (Math|Float|Clamp(Float) (+ (Variables|Default|GetCurrentHealth) IncomingHeal) 0.0 (Variables|Default|GetMaxHealth)))
    (Variables|/Script/UMG.ProgressBar|SetPercent (Variables|/Game/Widgets/WBP_PlayerHealthBar.WBP_PlayerHealthBar_C|GetProgressBarHealth _wbp_playerhealthbar) (Math|Float|SafeDivide (Variables|Default|GetCurrentHealth) (Variables|Default|GetMaxHealth)))
    (Variables|/Script/UMG.TextBlock|SetText (Variables|/Game/Widgets/WBP_PlayerHealthBar.WBP_PlayerHealthBar_C|GetTextBlock_Health _wbp_playerhealthbar) (Utilities|Text|ToText(Float) (Variables|Default|GetCurrentHealth) "HalfToEven"))
    (Variables|/Script/UMG.TextBlock|SetText (Variables|/Game/Widgets/WBP_PlayerHealthBar.WBP_PlayerHealthBar_C|GetTextBlock_MaxHealth _wbp_playerhealthbar) (Utilities|Text|ToText(Float) (Variables|Default|GetMaxHealth) "HalfToEven"))))

(fn IncreaseStamina
  (params (StaminaRecovered :type Float%20%28double-precision%29))
  (bind _bp_player_controller (Variables|Default|GetBP%20Player%20Controller))
  (bind _wbp_hud_overlay (Variables|/Game/Bluepints/BP_PlayerController.BP_PlayerController_C|GetWBP%20Hud%20Overlay _bp_player_controller))
  (bind _wbp_playestaminabar (Variables|/Game/Widgets/WBP_RPGHUD.WBP_RPGHUD_C|GetWBP_PlayeStaminaBar _wbp_hud_overlay))
  (if (not (>= (Variables|Default|GetCurrent%20Stamina) (Variables|Default|GetMaxHealth)))
    (Variables|Default|SetCurrent%20Stamina (Math|Float|Clamp(Float) (+ (Variables|Default|GetCurrent%20Stamina) StaminaRecovered) 0.0 (Variables|Default|GetMaxStamina)))
    (Variables|/Script/UMG.ProgressBar|SetPercent (Variables|/Game/Widgets/WBP_PlayeStaminaBar.WBP_PlayeStaminaBar_C|GetProgressBarStamina _wbp_playestaminabar) (Math|Float|SafeDivide (Variables|Default|GetCurrent%20Stamina) (Variables|Default|GetMaxStamina)))
    (Variables|/Script/UMG.TextBlock|SetText (Variables|/Game/Widgets/WBP_PlayeStaminaBar.WBP_PlayeStaminaBar_C|GetTextBlock_Stamina _wbp_playestaminabar) (Utilities|Text|ToText(Float) (Variables|Default|GetCurrent%20Stamina) "HalfToEven"))
    (Variables|/Script/UMG.TextBlock|SetText (Variables|/Game/Widgets/WBP_PlayeStaminaBar.WBP_PlayeStaminaBar_C|GetTextBlock_MaxStamina _wbp_playestaminabar) (Utilities|Text|ToText(Float) (Variables|Default|GetMaxStamina) "HalfToEven"))))

(fn DecreaseStamina
  (params (Staminaused :type Float%20%28double-precision%29))
  (bind _bp_player_controller (Variables|Default|GetBP%20Player%20Controller))
  (bind _wbp_hud_overlay (Variables|/Game/Bluepints/BP_PlayerController.BP_PlayerController_C|GetWBP%20Hud%20Overlay _bp_player_controller))
  (bind _wbp_playestaminabar (Variables|/Game/Widgets/WBP_RPGHUD.WBP_RPGHUD_C|GetWBP_PlayeStaminaBar _wbp_hud_overlay))
  (Variables|Default|SetCurrent%20Stamina (Math|Float|Clamp(Float) (- (Variables|Default|GetCurrent%20Stamina) Staminaused) 0.0 (Variables|Default|GetMaxStamina)))
  (Variables|/Script/UMG.ProgressBar|SetPercent (Variables|/Game/Widgets/WBP_PlayeStaminaBar.WBP_PlayeStaminaBar_C|GetProgressBarStamina _wbp_playestaminabar) (Math|Float|SafeDivide (Variables|Default|GetCurrent%20Stamina) (Variables|Default|GetMaxStamina)))
  (Variables|/Script/UMG.TextBlock|SetText (Variables|/Game/Widgets/WBP_PlayeStaminaBar.WBP_PlayeStaminaBar_C|GetTextBlock_Stamina _wbp_playestaminabar) (Utilities|Text|ToText(Float) (Variables|Default|GetCurrent%20Stamina) "HalfToEven"))
  (Variables|/Script/UMG.TextBlock|SetText (Variables|/Game/Widgets/WBP_PlayeStaminaBar.WBP_PlayeStaminaBar_C|GetTextBlock_MaxStamina _wbp_playestaminabar) (Utilities|Text|ToText(Float) (Variables|Default|GetMaxStamina) "HalfToEven"))
  (Variables|Default|SetNoStamina? (<= (Variables|Default|GetCurrent%20Stamina) 0.0))
  (return false))