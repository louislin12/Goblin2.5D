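; BP_Trap is a trap actor that rises when an RPG character comes near and damages whatever touches it.
; SenseBox overlap stores the BP_RPGChar_Base character and plays the raise animation; any end overlap, like BeginPlay, plays the lower animation.
; Spark overlap applies heavy damage to the overlapping actor, then calls the hit-react on the stored character, which may differ from that actor.
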(event OnComponentEndOverlap(SenseBox)
  (params (OverlappedComponent :type Primitive%20Component%20Object%20Reference) (OtherActor :type Actor%20Object%20Reference) (OtherComp :type Primitive%20Component%20Object%20Reference) (OtherBodyIndex :type Integer))
  (Components|Animation|PlayAnimation (Variables|Default|GetSkeletalMesh) "/Game/3DAssets/BlenderMesh/TRAPDown.TRAPDown" false))

(event OnComponentBeginOverlap(SenseBox)
  (params (OverlappedComponent :type Primitive%20Component%20Object%20Reference) (OtherActor :type Actor%20Object%20Reference) (OtherComp :type Primitive%20Component%20Object%20Reference) (OtherBodyIndex :type Integer) (bFromSweep :type Boolean) (SweepResult :type Hit%20Result%20Structure%20%28by%20ref%29))
  (bind _asbp_rpgchar_base (Utilities|Casting|CastToBP_RPGChar_Base OtherActor))
  (Variables|Default|SetAs%20BP%20RPGChar%20Base _asbp_rpgchar_base)
  (Components|Animation|PlayAnimation (Variables|Default|GetSkeletalMesh) "/Game/3DAssets/BlenderMesh/trapup.trapup" false))

(event OnComponentBeginOverlap(Spark)
  (params (OverlappedComponent :type Primitive%20Component%20Object%20Reference) (OtherActor :type Actor%20Object%20Reference) (OtherComp :type Primitive%20Component%20Object%20Reference) (OtherBodyIndex :type Integer) (bFromSweep :type Boolean) (SweepResult :type Hit%20Result%20Structure%20%28by%20ref%29))
  (bind _returnvalue (Game|Damage|ApplyDamage OtherActor 1e+02 0 0))
  (Default|GetHitPlayHitReactAnimation (Variables|Default|GetAs%20BP%20RPGChar%20Base) _returnvalue))

(event EventBeginPlay
  (Components|Animation|PlayAnimation (Variables|Default|GetSkeletalMesh) "/Game/3DAssets/BlenderMesh/TRAPDown.TRAPDown" false))

(event Collision|EventActorBeginOverlap
  (params (OtherActor :type Actor%20Object%20Reference)))

(event EventTick
  (params (DeltaSeconds :type Float%20%28single-precision%29)))

(fn ConstructionScript)