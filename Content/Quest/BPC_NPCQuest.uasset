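; NPC quest component that offers quests to the player and handles turning them in, using rows from the QuestList data table.
; ActivateQuest and FoundQuest check the player's quest component, then show NPC indicators, the cursor and accept or complete dialogue widgets.
; PositionWidget projects the speaker's location to screen space to place the accept widget.
; ConditionQuest completes Collect quests by item count and grants EXP; DropReward is an empty stub.
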(event EventBeginPlay)

(event EventTick
  (params (DeltaSeconds :type Float%20%28single-precision%29)))

(fn ActivateQuest
  (params (ID :type Array%20of%20Names) (NPC :type BP%20NPC%20Object%20Reference))
  (Variables|Default|SetNPC NPC)
  (bind _array_element (Utilities|Array|ForEachLoopwithBreak ID :!label _label)
    (:LoopBody
      (if (Utilities|Array|ContainsItem (Variables|/Game/Quest/BPC_PlayerQuestComponent.BPC_PlayerQuestComponent_C|GetActivate%20Quest (CallFunction|GetPlayerQuestComponent)) _array_element)
        _
        (else
          (bind _out_row (CallFunction|GetQuest _array_element))
          (Variables|Default|SetQuest%20Struct _out_row)))
      (if (== (.QuestPrerequisite (Utilities|Struct|BreakQuestStruct _out_row)) "")
        (Rendering|SetVisibility (Variables|/Game/Character_BP+AS/BP_NPC.BP_NPC_C|GetQuestacceptIndicator NPC) true false :!label _label_2)
        (Variables|/Script/Engine.PlayerController|SetbShowMouseCursor (Game|GetPlayerController 0) true)
        (Rendering|SetVisibility (Variables|/Game/Character_BP+AS/BP_RPGChar_Base.BP_RPGChar_Base_C|GetDialogueIndicator NPC) false false)
        (CallFunction|PositionWidget NPC)
        (Rendering|Components|TextRender|SetText (Variables|/Game/Widgets/WBP_AcceptQuest.WBP_AcceptQuest_C|GetQuestDialogue (Variables|/Game/Character_BP+AS/BP_NPC.BP_NPC_C|GetAs%20WBP%20Accept%20Quest NPC)) (.AcceptDialogue (Utilities|Struct|BreakQuestDialogue (.QuestDialogue (Utilities|Struct|BreakQuestStruct (Variables|Default|GetQuest%20Struct))))))
        (Variables|/Game/Widgets/WBP_AcceptQuest.WBP_AcceptQuest_C|SetID (Variables|/Game/Character_BP+AS/BP_NPC.BP_NPC_C|GetAs%20WBP%20Accept%20Quest NPC) (.ID (Utilities|Struct|BreakQuestDialogue (.QuestDialogue (Utilities|Struct|BreakQuestStruct (Variables|Default|GetQuest%20Struct))))))
        (goto _label Break)
        (elif (not (Utilities|Array|ContainsItem (Variables|/Game/Quest/BPC_PlayerQuestComponent.BPC_PlayerQuestComponent_C|GetComplete%20Quest (CallFunction|GetPlayerQuestComponent)) (.QuestPrerequisite (Utilities|Struct|BreakQuestStruct _out_row))))
          (goto _label_2))))))

(fn FoundQuest
  (params (NPCName :type String) (NPC :type BP%20NPC%20Object%20Reference))
  (bind _as_wbp_complete_quest (Variables|/Game/Character_BP+AS/BP_NPC.BP_NPC_C|GetAs%20WBP%20Complete%20Quest (Variables|Default|GetNPC)))
  (bind _array_element (Utilities|Array|ForEachLoopwithBreak (Variables|/Game/Quest/BPC_PlayerQuestComponent.BPC_PlayerQuestComponent_C|GetOngoing%20Quest (CallFunction|GetPlayerQuestComponent)))
    (:LoopBody
      (bind _out_row (CallFunction|GetQuest _array_element))
      (if (== NPCName (.ToWho (Utilities|Struct|BreakQuestDetail (.QuestDetail (Utilities|Struct|BreakQuestStruct _out_row)))))
        (Rendering|SetVisibility (Variables|/Game/Character_BP+AS/BP_NPC.BP_NPC_C|GetQuestcompleteIndicator (Variables|Default|GetNPC)) true false)
        (Variables|/Script/Engine.PlayerController|SetbShowMouseCursor (Game|GetPlayerController 0) true)
        (Rendering|SetVisibility (Variables|/Game/Character_BP+AS/BP_RPGChar_Base.BP_RPGChar_Base_C|GetDialogueIndicator (Variables|Default|GetNPC)) false false)
        (CallFunction|PositionWidget 0)
        (Rendering|Components|TextRender|SetText (Variables|/Game/Widgets/WBP_CompleteQuest1.WBP_CompleteQuest1_C|GetQuestCompleteDialogue _as_wbp_complete_quest) (.FinishDialogue (Utilities|Struct|BreakQuestDialogue (.QuestDialogue (Utilities|Struct|BreakQuestStruct _out_row)))))
        (Variables|/Game/Widgets/WBP_CompleteQuest1.WBP_CompleteQuest1_C|SetID _as_wbp_complete_quest (.ID (Utilities|Struct|BreakQuestDetail (.QuestDetail (Utilities|Struct|BreakQuestStruct _out_row)))))))))

(fn DropReward
  (params (Items :type Map%20of%20Names%20to%20Integers) (RareProbability :type Float%20%28double-precision%29) (NormalProbability :type Float%20%28double-precision%29))
  (return))

(fn ConditionQuest
  (params (ID :type Name))
  (bind _bpc_playerquestcomponent (CallFunction|GetPlayerQuestComponent))
  (bind _out_row (CallFunction|GetQuest ID))
  (switch Utilities|FlowControl|Switch|SwitchonQuestType (.QuestType (Utilities|Struct|BreakQuestDetail (.QuestDetail (Utilities|Struct|BreakQuestStruct _out_row))))
    (:NewEnumerator1
      (if (.ReturnValue (Utilities|Map|Find (Variables|/Game/Quest/BPC_PlayerQuestComponent.BPC_PlayerQuestComponent_C|GetQuest%20Item (CallFunction|GetPlayerQuestComponent)) (Utilities|String|StringToName (.TargetWho (Utilities|Struct|BreakQuestDetail (.QuestDetail (Utilities|Struct|BreakQuestStruct _out_row)))))))
        (if (>= (.Value (Utilities|Map|Find (Variables|/Game/Quest/BPC_PlayerQuestComponent.BPC_PlayerQuestComponent_C|GetQuest%20Item (CallFunction|GetPlayerQuestComponent)) (Utilities|String|StringToName (.TargetWho (Utilities|Struct|BreakQuestDetail (.QuestDetail (Utilities|Struct|BreakQuestStruct _out_row))))))) (.RequiredAmount (Utilities|Struct|BreakQuestDetail (.QuestDetail (Utilities|Struct|BreakQuestStruct _out_row)))))
          (Default|AddCompleteQuest _bpc_playerquestcomponent ID)
          (Utilities|Array|RemoveItem (Variables|/Game/Quest/BPC_PlayerQuestComponent.BPC_PlayerQuestComponent_C|GetOngoing%20Quest _bpc_playerquestcomponent) ID)
          (Default|GainEXP (CallFunction|GetPlayerStats) (.EXPOffer (Utilities|Struct|BreakQuestDetail (.QuestDetail (Utilities|Struct|BreakQuestStruct _out_row)))))
          (if (not (== (Utilities|Map|Length (.Rewards (Utilities|Struct|BreakQuestDetail (.QuestDetail (Utilities|Struct|BreakQuestStruct _out_row))))) 0))
            (CallFunction|DropReward (.Rewards (Utilities|Struct|BreakQuestDetail (.QuestDetail (Utilities|Struct|BreakQuestStruct _out_row)))) (.RareProbability (Utilities|Struct|BreakQuestDetail (.QuestDetail (Utilities|Struct|BreakQuestStruct _out_row)))) (.NormalProbability (Utilities|Struct|BreakQuestDetail (.QuestDetail (Utilities|Struct|BreakQuestStruct _out_row)))))
            (if true
              _)))))))

(fn GetQuest
  (params (RowName :type Name))
  (bind _returnvalue (Utilities|GetDataTableRow "/Game/DataTable/QuestList.QuestList" RowName)
    (:then
      (return _returnvalue))))

(fn PositionWidget
  (params (Speaking%20Actor :type Actor%20Object%20Reference))
  (bind _npc (Variables|Default|GetNPC))
  (bind _as_wbp_accept_quest (Variables|/Game/Character_BP+AS/BP_NPC.BP_NPC_C|GetAs%20WBP%20Accept%20Quest _npc))
  (bind _returnvalue (Class|Widget|GetDesiredSize _as_wbp_accept_quest))
  (Class|Widget|ForceLayoutPrepass (Variables|/Game/Character_BP+AS/BP_NPC.BP_NPC_C|GetAs%20WBP%20Accept%20Quest (Variables|Default|GetNPC)))
  (Class|CanvasPanelSlot|SetPosition (Class|WidgetLayoutLibrary|SlotasCanvasSlot (Variables|/Game/Character_BP+AS/BP_NPC.BP_NPC_C|GetAs%20WBP%20Accept%20Quest (Variables|Default|GetNPC))) (Utilities|Operators|Subtract (.ScreenPosition (Class|WidgetLayoutLibrary|ProjectWorldLocationtoWidgetPosition (Game|GetPlayerController 0) (Transformation|GetActorLocation Speaking%20Actor) false)) (Math|Vector2D|MakeVector2D (/ (.x _returnvalue) 2.0) (.y _returnvalue)) (Variables|Default|GetOffset))))