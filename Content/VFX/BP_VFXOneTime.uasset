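; A one-shot 2D visual effect actor that plays a Paper2D flipbook once and then removes itself.
; On BeginPlay it assigns the VFXFlipbook variable to its flipbook component, disables looping and sets a custom lit sprite material on the first slot.
; When the flipbook finishes playing, the actor destroys itself.
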(event OnFinishedPlaying(PaperFlipbook)
  (Actor|DestroyActor))

(event EventBeginPlay
  (Sprite|SetFlipbook (Variables|Default|GetPaperFlipbook) (Variables|Default|GetVFXFlipbook))
  (Components|Timeline|SetLooping (Variables|Default|GetPaperFlipbook) false)
  (Rendering|Material|SetMaterial (Variables|Default|GetPaperFlipbook) 0 0)
  (Rendering|Material|SetMaterial (Variables|Default|GetPaperFlipbook) 0 "/Game/Materials/M_CustomLitSpriteMaterial_Inst.M_CustomLitSpriteMaterial_Inst"))

(event Collision|EventActorBeginOverlap
  (params (OtherActor :type Actor%20Object%20Reference)))

(event EventTick
  (params (DeltaSeconds :type Float%20%28single-precision%29)))

(fn ConstructionScript)