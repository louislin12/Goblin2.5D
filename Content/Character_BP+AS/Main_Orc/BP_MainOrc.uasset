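; BP_MainOrc is the main orc character Blueprint, handling the normal attack input with PaperZD-style animation.
; Pressing attack halts movement and triggers HitStop, then jumps to a Spinning node when hopping or plays an ATK override otherwise.
; IsPunching blocks re-entry until the override completes or cancels, but clears immediately in the hopping branch.
; Walking attacks zero walk speed, and releasing the input restores it.
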(event Input|EnhancedActionEvents|EnhancedInputActionIA_NormalATK
  (params (ActionValue :type Boolean) (ElapsedSeconds :type Float%20%28double-precision%29) (TriggeredSeconds :type Float%20%28double-precision%29) (InputAction :type Input%20Action%20Object%20Reference :default "/Game/Input/Actions/IA_NormalATK.IA_NormalATK"))
  (:Started
    ;[0 0 0] Punch
    (if (not (Variables|Default|GetIsPunching?))
      (if (Variables|Default|GetIsWalking?)
        (Variables|/Script/Engine.CharacterMovementComponent|SetMaxWalkSpeed (Variables|Character|GetCharacterMovement) 0.0))
      (if (Variables|Default|GetIsHopping?)
        (Variables|Default|SetIsPunching? true)
        (Class|PaperZDAnimInstance|JumptoNode (Variables|/Script/PaperZD.PaperZDAnimationComponent|GetAnimInstance (Variables|Default|GetAnimationComponent)) "Spinning" "None")
        (Components|Movement|StopMovementImmediately (Variables|Character|GetCharacterMovement))
        (CallFunction|HitStop)
        (Variables|Default|SetIsPunching? false)
        (else
          (Components|Movement|StopMovementImmediately (Variables|Character|GetCharacterMovement))
          (CallFunction|HitStop)
          (|PlayAnimationOverridewithCallbacks (Variables|/Script/PaperZD.PaperZDAnimationComponent|GetAnimInstance (Variables|Default|GetAnimationComponent)) "/Game/Character_BP+AS/Main_Orc/AnimSequences/ATK.ATK" "DefaultSlot" 1.0 0.0
            (:then
              (Variables|Default|SetIsPunching? true))
            (:OnCompleted
              (Variables|Default|SetIsPunching? false :!label _label))
            (:OnCancelled
              (goto _label)))))))
  (:Completed
    (Variables|/Script/Engine.CharacterMovementComponent|SetMaxWalkSpeed (Variables|Character|GetCharacterMovement) 6e+02)))

(event EventBeginPlay
  (|CallParentFunction) ; This node is disabled and will not be called.\nDrag off pins to build functionality.
)

(event Collision|EventActorBeginOverlap
  (params (OtherActor :type Actor%20Object%20Reference))
  (|CallParentFunction OtherActor) ; This node is disabled and will not be called.\nDrag off pins to build functionality.
)

(event EventTick
  (params (DeltaSeconds :type Float%20%28single-precision%29))
  (|CallParentFunction DeltaSeconds) ; This node is disabled and will not be called.\nDrag off pins to build functionality.
)

(fn ConstructionScript
  (|CallParentFunction))