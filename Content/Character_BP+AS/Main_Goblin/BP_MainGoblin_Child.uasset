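; Child Blueprint of the main goblin character that maps attack and block/eat inputs to PaperZD animations.
; Normal attack plays a punch override, or jumps the state machine to Spinning while hopping.
; Block/eat plays mouth open, loop and close overrides across input phases, gated by the CheckCondition macro.
; IsPunching locks out new actions and clears when overrides complete or cancel; the spin branch never clears it here.
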(event Input|EnhancedActionEvents|EnhancedInputActionIA_BlockEat
  (params (ActionValue :type Boolean) (ElapsedSeconds :type Float%20%28double-precision%29) (TriggeredSeconds :type Float%20%28double-precision%29) (InputAction :type Input%20Action%20Object%20Reference :default "/Game/Input/Actions/IA_BlockEat.IA_BlockEat"))
  (:Triggered
    (Utilities|CheckCondition
      (:else
        (|PlayAnimationOverridewithCallbacks (Variables|/Script/PaperZD.PaperZDAnimationComponent|GetAnimInstance (Variables|Default|GetAnimationComponent)) "/Game/Character_BP+AS/Main_Goblin/MainGoblin/AnimSequences/MouthOpen.MouthOpen" "DefaultSlot" 1.0 0.0
          (:then
            (Variables|Default|SetIsPunching? true))
          (:OnCompleted
            (Variables|Default|SetIsPunching? false :!label _label))
          (:OnCancelled
            (goto _label))))))
  (:Ongoing
    (Utilities|CheckCondition
      (:else
        (|PlayAnimationOverridewithCallbacks (Variables|/Script/PaperZD.PaperZDAnimationComponent|GetAnimInstance (Variables|Default|GetAnimationComponent)) "/Game/Character_BP+AS/Main_Goblin/MainGoblin/AnimSequences/MouthLoop.MouthLoop" "DefaultSlot" 1.0 0.0
          (:then
            (Variables|Default|SetIsPunching? true))
          (:OnCompleted
            (Variables|Default|SetIsPunching? false :!label _label_2))
          (:OnCancelled
            (goto _label_2))))))
  (:Completed
    (Utilities|CheckCondition
      (:else
        (|PlayAnimationOverridewithCallbacks (Variables|/Script/PaperZD.PaperZDAnimationComponent|GetAnimInstance (Variables|Default|GetAnimationComponent)) "/Game/Character_BP+AS/Main_Goblin/MainGoblin/AnimSequences/MouthClose.MouthClose" "DefaultSlot" 1.0 0.0
          (:then
            (Variables|Default|SetIsPunching? true))
          (:OnCompleted
            (Variables|Default|SetIsPunching? false :!label _label_3))
          (:OnCancelled
            (goto _label_3)))))))

(event Input|EnhancedActionEvents|EnhancedInputActionIA_NormalATK
  (params (ActionValue :type Boolean) (ElapsedSeconds :type Float%20%28double-precision%29) (TriggeredSeconds :type Float%20%28double-precision%29) (InputAction :type Input%20Action%20Object%20Reference :default "/Game/Input/Actions/IA_NormalATK.IA_NormalATK"))
  ;[0 0 0] Punch
  (:Started
    (if (not (Variables|Default|GetIsPunching?))
      (if (Variables|Default|GetGoblinAnimation?)
        (if (Variables|Default|GetIsHopping?)
          (Class|PaperZDAnimInstance|JumptoNode (Variables|/Script/PaperZD.PaperZDAnimationComponent|GetAnimInstance (Variables|Default|GetAnimationComponent)) "Spinning" "None")
          (Variables|Default|SetIsPunching? true)
          (else
            (|PlayAnimationOverridewithCallbacks (Variables|/Script/PaperZD.PaperZDAnimationComponent|GetAnimInstance (Variables|Default|GetAnimationComponent)) "/Game/Character_BP+AS/Main_Goblin/MainGoblin/AnimSequences/Punch.Punch" "DefaultSlot" 1.0 0.0
              (:then
                (Variables|Default|SetIsPunching? true))
              (:OnCompleted
                (Variables|Default|SetIsPunching? false :!label _label))
              (:OnCancelled
                (goto _label)))))))))

(event Collision|EventActorBeginOverlap
  (params (OtherActor :type Actor%20Object%20Reference))
  (|CallParentFunction OtherActor) ; This node is disabled and will not be called.\nDrag off pins to build functionality.
)

(event EventTick
  (params (DeltaSeconds :type Float%20%28single-precision%29))
  (|CallParentFunction DeltaSeconds) ; This node is disabled and will not be called.\nDrag off pins to build functionality.
)

(fn ConstructionScript
  (|CallParentFunction))