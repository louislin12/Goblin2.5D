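; Main Spirit character Blueprint that adds energy-limited flight and a hurt-reaction animation.
; Space toggles between Flying and Falling movement, while IA_Fly adds vertical movement and drains frame-time-scaled energy as long as the energy check passes.
; Running out or toggling off switches to Falling and resets energy to a fixed amount.
; A health-driven event plays the hurt reaction as an animation override.
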(event Input|EnhancedActionEvents|EnhancedInputActionIA_Fly
  (params (ActionValue :type Vector%202D%20Structure) (ElapsedSeconds :type Float%20%28double-precision%29) (TriggeredSeconds :type Float%20%28double-precision%29) (InputAction :type Input%20Action%20Object%20Reference :default "/Game/Input/Actions/IA_Fly.IA_Fly"))
  (if (Class|NavMovementComponent|IsFlying (Variables|Character|GetCharacterMovement))
    (bind _hasenergy (Class|BPIStamina|HasEnergy(Message) self))
    (if _hasenergy
      (Pawn|Input|AddMovementInput (* (Transformation|GetActorUpVector (Game|GetPlayerCharacter 0)) (Variables|Default|GetFlyHeightAmount)) (.x ActionValue) false)
      (CallFunction|DrainEnergy)
      (else
        (Pawn|Components|CharacterMovement|SetMovementMode (Variables|Character|GetCharacterMovement) "MOVE_Falling" 0)
        (Variables|Default|SetFlyHeightEnergy 5e+01)))))

(event EventBeginPlay
  (|CallParentFunction))

(event Collision|EventActorBeginOverlap
  (params (OtherActor :type Actor%20Object%20Reference))
  (|CallParentFunction OtherActor) ; This node is disabled and will not be called.\nDrag off pins to build functionality.
)

(event EventDrainEnergy
  (CallFunction|ConsumeEnergyforFrame))

(event EventPlayAnimBaseonHealth
  (Class|PaperZDAnimInstance|PlayAnimationOverride (Variables|/Script/PaperZD.PaperZDAnimationComponent|GetAnimInstance (Variables|Default|GetAnimationComponent)) (Variables|Default|GetHurt%20React%20Anim%20Sequence) "DefaultSlot" 1.0 0.0))

(event Input|KeyboardEvents|SpaceBar
  (params (Key :type Key%20Structure))
  (:Pressed
    (Utilities|FlowControl|FlipFlop
      (:A
        (Pawn|Components|CharacterMovement|SetMovementMode (Variables|Character|GetCharacterMovement) "MOVE_Flying" 0)
        (CallFunction|DrainEnergy))
      (:B
        (Pawn|Components|CharacterMovement|SetMovementMode (Variables|Character|GetCharacterMovement) "MOVE_Falling" 0)
        (Variables|Default|SetFlyHeightEnergy 5e+01)))))

(fn ConstructionScript
  (|CallParentFunction))

(fn ConsumeEnergyforFrame
  (Variables|Default|SetFlyHeightEnergy (Math|Float|Clamp(Float) (- (Variables|Default|GetFlyHeightEnergy) (* (Variables|Default|GetEnergyDrainRate) (Utilities|Time|GetWorldDeltaSeconds))) 0.0 (Variables|Default|GetMaxEnergy))))

(fn HasEnergy
  (return (> (Variables|Default|GetFlyHeightEnergy) 0.0)))