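; Player-controlled Paper2D RPG character with a debug-style key toggle between goblin and orc forms by swapping flipbook and anim instance.
; BeginPlay restores health from the GameInstance by character type and starts the first quest.
; Enhanced Input drives movement, inventory UI and timer-based stamina sprint, while a per-tick sphere trace selects the target for interface-message interaction.
; Stats, inventory and quest components are exposed through getters; radial force components supply punch and spin-attack impulses.
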(event Custom|Transform%20to%20Orc
  ;[0 0 0] Old Transform Can delete. Use only if need to all in one blueprint
  (Sprite|SetFlipbook (Variables|Default|GetSprite) "/Game/PaperAssets/Orc_GTransform/orc1_idle_body-sheet__IDLE_D.orc1_idle_body-sheet__IDLE_D")
  (Class|PaperZDAnimationComponent|SetAnimInstanceClass (Variables|Default|GetAnimationComponent) "/Game/Character_BP+AS/Main_Orc/ABP_MainOrc.ABP_MainOrc_C")
  (Variables|ActionLocked|SetGoblinAnimation? false)
  (Variables|ActionLocked|SetOrcAnimation? true)
  (if (Variables|ActionLocked|GetFrom%20Goblin?)
    (Variables|ActionLocked|SetFrom%20Goblin? false)
    (Transformation|SetWorldTransform (Variables|Default|GetSprite) (Math|Transform|MakeTransform (- (Transformation|GetWorldLocation (Variables|Default|GetSprite)) "0.000000,0.000000,94.000000") "0, 0, 0" "1.000000,1.000000,1.000000") false false)))

(event EventOnHealthChanged
  (params (CurrentHealth :type Float%20%28double-precision%29) (MaxHealth :type Float%20%28double-precision%29))
  (|CallParentFunction CurrentHealth MaxHealth)
  (Class|BPICharacterInterace|UpdateHealthWidget(Message) (Game|GetPlayerController 0) CurrentHealth MaxHealth))

(event Collision|EventActorBeginOverlap
  (params (OtherActor :type Actor%20Object%20Reference))
  (|CallParentFunction OtherActor) ; This node is disabled and will not be called.\nDrag off pins to build functionality.
)

(event EventPossessed
  (params (NewController :type Controller%20Object%20Reference))
  (bind _asbp_player_controller (Utilities|Casting|CastToBP_PlayerController (Pawn|GetController)))
  (bind _output_get (Variables|Default|SetAs%20BP%20Player%20Controller _asbp_player_controller))
  (Input|AddMappingContext (PlayerController|LocalPlayerSubsystems|GetEnhancedInputLocalPlayerSubsystem _output_get) "/Game/Input/IMC_RPG.IMC_RPG" 0 "(bIgnoreAllPressedKeysUntilRelease=True,bForceImmediately=False,bNotifyUserSettings=False)"))

(event EventHandleDeath
  (bind _returnvalue (Game|GetPlayerController 0))
  (Input|SetInputModeUIOnly _returnvalue 0 "DoNotLock" false)
  (Variables|/Script/Engine.PlayerController|SetbShowMouseCursor _returnvalue true))

(event EventBeginPlay
  (bind _bpc_stats (Variables|Default|GetBPC_Stats))
  (bind _bpc_stats_2 (Variables|Default|GetBPC_Stats))
  (|CallParentFunction)
  (Utilities|FlowControl|Sequence
    (:then_0
      (Class|PlayerController|SetAudioListenerOverride (Game|GetPlayerController 0) (Variables|Default|GetSprite) "0, 0, 0" "0.000000,270.000000,0.000000")
      (bind _characterhealth (Class|BPIGameInstance|GetCharacterSavedHealth(Message) (Game|GetGameInstance)))
      (if (.ReturnValue (Utilities|Map|Find _characterhealth (Variables|Default|GetCharacterType)))
        (Variables|/Game/Components/BPC_Stats.BPC_Stats_C|SetCurrentHealth _bpc_stats_2 (.Value (Utilities|Map|Find _characterhealth (Variables|Default|GetCharacterType))))
        (Default|AddValuetoHealth _bpc_stats_2 0.0)
        (else
          (Default|AddValuetoHealth _bpc_stats (Variables|/Game/Components/BPC_Stats.BPC_Stats_C|GetMaxHealth _bpc_stats)))))
    (:then_1
      (Utilities|FlowControl|Delay 2.0)
      (Default|BeginQuest (Variables|Default|GetBPC_QuestComponent) (Game|GetPlayerController 0) "/Game/Core/Blueprints/Quests/Quests/DA_Quest_01_SRAKA.DA_Quest_01_SRAKA"))))

(event Input|KeyboardEvents|P
  (params (Key :type Key%20Structure :default "None"))
  ;[0 0 0] Old Transform Can delete. Use only if need to all in one blueprint
  (:Pressed
    (if (not (Variables|Combat|GetIsPunching?))
      (Utilities|FlowControl|FlipFlop
        (:A
          (Sprite|SetFlipbook (Variables|Default|GetSprite) "/Game/PaperAssets/Orc_GTransform/orc1_idle_body-sheet__IDLE_D.orc1_idle_body-sheet__IDLE_D")
          (Class|PaperZDAnimationComponent|SetAnimInstanceClass (Variables|Default|GetAnimationComponent) "/Game/Character_BP+AS/Main_Orc/ABP_MainOrc.ABP_MainOrc_C")
          (Variables|ActionLocked|SetGoblinAnimation? false)
          (Variables|ActionLocked|SetOrcAnimation? true)
          (if (Variables|ActionLocked|GetFrom%20Goblin?)
            (Variables|ActionLocked|SetFrom%20Goblin? false)
            (Transformation|SetWorldTransform (Variables|Default|GetSprite) (Math|Transform|MakeTransform (- (Transformation|GetWorldLocation (Variables|Default|GetSprite)) "0.000000,0.000000,94.000000") "0, 0, 0" "1.000000,1.000000,1.000000") false false)))
        (:B
          (Sprite|SetFlipbook (Variables|Default|GetSprite) "/Game/PaperAssets/Main_Goblin/gobu_Idle__IDLE_D1.gobu_Idle__IDLE_D1")
          (Class|PaperZDAnimationComponent|SetAnimInstanceClass (Variables|Default|GetAnimationComponent) "/Game/Character_BP+AS/Main_Goblin/MainGoblin/ABP_Maingoblin.ABP_Maingoblin_C")
          (Variables|ActionLocked|SetGoblinAnimation? true)
          (Variables|ActionLocked|SetOrcAnimation? false)
          (Variables|ActionLocked|SetFrom%20Goblin? true)
          (Transformation|SetWorldTransform (Variables|Default|GetSprite) (Math|Transform|MakeTransform (+ (Transformation|GetWorldLocation (Variables|Default|GetSprite)) "0.000000,0.000000,94.000000") "0, 0, 0" "1.000000,1.000000,1.000000") false false))))))

(event Custom|Use%20Stamina
  ;[0 0 0] Sprint and Stamina USE
  (Default|DecreaseStamina (Variables|Default|GetBPC_Stats) 1.0))

(event Custom|RecoverStamina
  (bind _bpc_stats (Variables|Default|GetBPC_Stats))
  ;[0 0 0] Sprint and Stamina USE
  (Default|IncreaseStamina _bpc_stats 1.0)
  (Variables|/Game/Components/BPC_Stats.BPC_Stats_C|SetNoStamina? _bpc_stats false))

(event Input|EnhancedActionEvents|EnhancedInputActionIA_Move
  (params (ActionValue :type Vector%202D%20Structure) (ElapsedSeconds :type Float%20%28double-precision%29) (TriggeredSeconds :type Float%20%28double-precision%29) (InputAction :type Input%20Action%20Object%20Reference :default "/Game/Input/Actions/IA_Move.IA_Move"))
  (bind (_x _y) (Math|Vector2D|BreakVector2D ActionValue))
  ;[0 0 0] Move
  (:Triggered
    (if (not (Variables|Default|GetIsInteractionLocked))
      (if (not (Variables|Combat|GetIsPunching?))
        (Pawn|Input|AddMovementInput "1.000000,0.000000,0.000000" _x false)
        (Pawn|Input|AddMovementInput "0.000000,1.000000,0.000000" _y false)
        (Variables|ActionLocked|SetIsWalking? true))))
  (:Completed
    (Variables|ActionLocked|SetIsWalking? false)))

(event Input|EnhancedActionEvents|EnhancedInputActionIA_Hop
  (params (ActionValue :type Boolean) (ElapsedSeconds :type Float%20%28double-precision%29) (TriggeredSeconds :type Float%20%28double-precision%29) (InputAction :type Input%20Action%20Object%20Reference :default "/Game/Input/Actions/IA_Hop.IA_Hop"))
  (bind _charactermovement (Variables|Character|GetCharacterMovement))
  ;[0 0 0] Sprint and Stamina USE
  (:Triggered
    (if (Variables|/Game/Components/BPC_Stats.BPC_Stats_C|GetNoStamina? (Variables|Default|GetBPC_Stats))
      (Variables|/Script/Engine.CharacterMovementComponent|SetMaxWalkSpeed _charactermovement (Variables|Default|GetInitial%20Walk%20Speed) :!label _label)
      (Variables|ActionLocked|SetIsHopping? false)
      (Utilities|Time|ClearandInvalidateTimerbyHandle (Variables|Default|GetStaminaTimer))
      (Utilities|FlowControl|Delay 2.0)
      (bind _returnvalue (Utilities|Time|SetTimerbyEvent (delegate Custom|RecoverStamina) 0.2 true))
      (Variables|Default|SetStaminaRecoverTimer _returnvalue)))
  (:Started
    (if (Variables|ActionLocked|GetFlyActivated?)
      (Variables|/Script/Engine.CharacterMovementComponent|SetMaxWalkSpeed _charactermovement (Variables|Default|GetMax%20Walk%20Speed))
      (Variables|ActionLocked|SetIsHopping? true)
      (Utilities|Time|ClearandInvalidateTimerbyHandle (Variables|Default|GetStaminaRecoverTimer))
      (bind _returnvalue_2 (Utilities|Time|SetTimerbyEvent (delegate Custom|Use%20Stamina) 0.2 true))
      (Variables|Default|SetStaminaTimer _returnvalue_2)))
  (:Completed
    (goto _label)))

(event Input|EnhancedActionEvents|EnhancedInputActionIA_Inventory
  (params (ActionValue :type Boolean) (ElapsedSeconds :type Float%20%28double-precision%29) (TriggeredSeconds :type Float%20%28double-precision%29) (InputAction :type Input%20Action%20Object%20Reference :default "/Game/Input/Actions/IA_Inventory.IA_Inventory"))
  (bind _returnvalue (Game|GetPlayerController 0))
  ;[0 0 0] Inventory
  (:Started
    (bind _returnvalue_2 (UserInterface|CreateWidget "/Game/Core/UI/Widgets/WBP_Inventory.WBP_Inventory_C"))
    (bind _output_get (Variables|Default|SetInventoryWidget _returnvalue_2))
    (UserInterface|Viewport|AddtoViewport _output_get 0)
    (Variables|/Script/Engine.PlayerController|SetbShowMouseCursor _returnvalue true)
    (Input|SetInputModeUIOnly _returnvalue (Variables|Default|GetInventoryWidget) "DoNotLock" false)))

(event Input|EnhancedActionEvents|EnhancedInputActionIA_Interact
  (params (ActionValue :type Boolean) (ElapsedSeconds :type Float%20%28double-precision%29) (TriggeredSeconds :type Float%20%28double-precision%29) (InputAction :type Input%20Action%20Object%20Reference :default "/Game/Input/Actions/IA_Interact.IA_Interact"))
  ;[0 0 0] Interact
  (:Started
    (if (not (Variables|Default|GetIsInteractionLocked))
      (bind _interactableobject (Variables|Default|GetInteractableObject)
        (:then
          (Class|BPIInteraction|Interact(Message) _interactableobject self))
        (:else)))))

(event Input|KeyboardEvents|Add
  (params (Key :type Key%20Structure))
  ;[0 0 0] Debug
  (:Pressed
    (Default|AddValuetoHealth (Variables|Default|GetBPC_Stats) 1e+01)))

(event EventTick
  (params (DeltaSeconds :type Float%20%28single-precision%29))
  (|CallParentFunction DeltaSeconds)
  (CallFunction|CheckforInteraction false 2e+02))

(fn ConstructionScript
  (|CallParentFunction))

(fn ApplyPunchForce
  (Class|RadialForceComponent|FireImpulse (Variables|Default|GetRadialForce%20PUNCH)))

(fn ApplySpinATk
  (Class|RadialForceComponent|FireImpulse (Variables|Default|GetRadialForce%20SPINATK)))

(fn FlipPaperAssetswithAcceleration
  (bind _returnvalue (Pawn|GetController))
  (Math|Float|CompareFloat (.x (Pawn|Components|CharacterMovement|GetCurrentAcceleration (Variables|Character|GetCharacterMovement))) 0.0
    (:>
      (Pawn|SetControlRotation _returnvalue (Math|Rotator|MakeRotator 0.0 0.0 0.0)))
    (:<
      (Pawn|SetControlRotation _returnvalue (Math|Rotator|MakeRotator 0.0 0.0 1.8e+02)))))

(fn CheckforInteraction
  (params (TraceComplex :type Boolean) (Radius :type Float%20%28double-precision%29))
  (bind _returnvalue (Game|GetPlayerCharacter 0))
  (bind _returnvalue_2 (Transformation|GetActorLocation _returnvalue))
  (bind _returnvalue_3 (- _returnvalue_2 "0.000000,0.000000,30.000000"))
  (bind _returnvalue_4 (Class|AGRInventoryComponent|GetAllItems (Variables|Default|GetBPC_Inventory)))
  (bind _output_get (LocalVariables|SetIgnoreTargets _returnvalue_4))
  (Utilities|Array|AppendArray _output_get (Utilities|Array|MakeArray (Variables|Default|GetInstigator)))
  (bind (_outhit _returnvalue_5) (Collision|SphereTraceByChannel _returnvalue_3 _returnvalue_3 Radius "TraceTypeQuery3" TraceComplex (LocalVariables|GetIgnoreTargets) "ForOneFrame" true "(R=0.503047,G=0.528093,B=1.000000,A=1.000000)"))
  (if _returnvalue_5
    (Utilities|IsValid (.HitActor (Collision|BreakHitResult _outhit))
      (:Is%20Valid
        (Variables|Default|SetInteractableObject (.HitActor (Collision|BreakHitResult _outhit))))
      (:Is%20Not%20Valid
        (Variables|Default|SetInteractableObject (.HitActor (Collision|BreakHitResult _outhit)) :!label _label)))
    (else
      (goto _label))))

(fn GetCharacterType
  (return (Variables|Default|GetCharacterType)))

(fn GetHealth
  (return (Variables|/Game/Components/BPC_Stats.BPC_Stats_C|GetCurrentHealth (Variables|Default|GetBPC_Stats))))

(fn GetInventoryComponent
  (return (Variables|Default|GetBPC_Inventory)))

(fn GetInventoryWidget
  (return (Variables|Default|GetInventoryWidget)))

(fn GetPlayerHUD
  (return 0))

(fn GetQuestComponent
  (return (Variables|Default|GetBPC_QuestComponent)))

(fn GetStatsComponent
  (return (Variables|Default|GetBPC_Stats)))

(fn HasEnergy
  (return false))