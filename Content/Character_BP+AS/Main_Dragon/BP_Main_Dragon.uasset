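; Player dragon character with PaperZD-style sprite animation, handling four-way movement, melee attacks, hopping and flight.
; Enhanced Input drives movement through a direction macro that moves only along the last recorded input, gated by interaction and punch flags.
; Normal attack stops movement and triggers hit stop, playing a melee override or jumping to a spin while hopping.
; Space toggles Flying and Falling, with a timeline lifting components on takeoff; hop boosts speed while flying.
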(event Input|EnhancedActionEvents|EnhancedInputActionIA_Fly
  (params (ActionValue :type Vector%202D%20Structure) (ElapsedSeconds :type Float%20%28double-precision%29) (TriggeredSeconds :type Float%20%28double-precision%29) (InputAction :type Input%20Action%20Object%20Reference :default "/Game/Input/Actions/IA_Fly.IA_Fly"))
  (if (Class|NavMovementComponent|IsFlying (Variables|Character|GetCharacterMovement))
    (Pawn|Input|AddMovementInput (* (Transformation|GetActorUpVector (Game|GetPlayerCharacter 0)) (Variables|Default|GetFlyHeightAmount)) (.x ActionValue) false)))

(event Input|EnhancedActionEvents|EnhancedInputActionIA_Move
  (params (ActionValue :type Vector%202D%20Structure) (ElapsedSeconds :type Float%20%28double-precision%29) (TriggeredSeconds :type Float%20%28double-precision%29) (InputAction :type Input%20Action%20Object%20Reference :default "/Game/Input/Actions/IA_Move.IA_Move"))
  ;[0 0 0] Disabled
)

(event Input|EnhancedActionEvents|EnhancedInputActionIA_Hop
  (params (ActionValue :type Boolean) (ElapsedSeconds :type Float%20%28double-precision%29) (TriggeredSeconds :type Float%20%28double-precision%29) (InputAction :type Input%20Action%20Object%20Reference :default "/Game/Input/Actions/IA_Hop.IA_Hop"))
  (bind _charactermovement (Variables|Character|GetCharacterMovement))
  (:Started
    (if (Variables|Default|GetFlyActivated?)
      (Variables|/Script/Engine.CharacterMovementComponent|SetMaxWalkSpeed _charactermovement 1.1e+03)
      (Variables|Default|SetIsHopping? true)))
  (:Completed
    (Variables|/Script/Engine.CharacterMovementComponent|SetMaxWalkSpeed _charactermovement 7.5e+02)
    (Variables|Default|SetIsHopping? false)))

(event Input|EnhancedActionEvents|EnhancedInputActionIA_NormalATK
  (params (ActionValue :type Boolean) (ElapsedSeconds :type Float%20%28double-precision%29) (TriggeredSeconds :type Float%20%28double-precision%29) (InputAction :type Input%20Action%20Object%20Reference :default "/Game/Input/Actions/IA_NormalATK.IA_NormalATK"))
  (:Started
    ;[0 0 0] Punch
    (if (not (Variables|Default|GetIsPunching?))
      (if (not (Variables|Default|GetIsWalking?))
        (if (Variables|Default|GetIsHopping?)
          (Variables|Default|SetIsPunching? true)
          (Class|PaperZDAnimInstance|JumptoNode (Variables|/Script/PaperZD.PaperZDAnimationComponent|GetAnimInstance (Variables|Default|GetAnimationComponent)) "Spinning" "None")
          (Components|Movement|StopMovementImmediately (Variables|Character|GetCharacterMovement))
          (CallFunction|HitStop)
          (Variables|Default|SetIsPunching? false)
          (elif (not (Variables|Default|GetFlyActivated?))
            (Components|Movement|StopMovementImmediately (Variables|Character|GetCharacterMovement))
            (CallFunction|HitStop)
            (|PlayAnimationOverridewithCallbacks (Variables|/Script/PaperZD.PaperZDAnimationComponent|GetAnimInstance (Variables|Default|GetAnimationComponent)) "/Game/Character_BP+AS/Main_Dragon/AnimSequences/Melee.Melee" "DefaultSlot" 1.0 0.0
              (:then
                (Variables|Default|SetIsPunching? true))
              (:OnCompleted
                (Variables|Default|SetIsPunching? false :!label _label))
              (:OnCancelled
                (goto _label)))))))))

(event Input|EnhancedActionEvents|EnhancedInputActionIA_Left
  (params (ActionValue :type Boolean) (ElapsedSeconds :type Float%20%28double-precision%29) (TriggeredSeconds :type Float%20%28double-precision%29) (InputAction :type Input%20Action%20Object%20Reference :default "/Game/Input/Actions/IA_Left.IA_Left"))
  (:Triggered
    (if (not (Variables|Default|GetIsInteractionLocked))
      (if (not (Variables|Default|GetIsPunching?))
        (Utilities|HandleDirectionInput (Utilities|Enum|LiteralenumE_RetroMovement "NewEnumerator1") "-1.000000,0.000000,0.000000" :!label _label)
        (Variables|Default|SetIsWalking? true))))
  (:Started
    (goto _label Started))
  (:Completed
    (Variables|Default|SetIsWalking? false)
    (goto _label Completed)))

(event Input|EnhancedActionEvents|EnhancedInputActionIA_Up
  (params (ActionValue :type Boolean) (ElapsedSeconds :type Float%20%28double-precision%29) (TriggeredSeconds :type Float%20%28double-precision%29) (InputAction :type Input%20Action%20Object%20Reference :default "/Game/Input/Actions/IA_Up.IA_Up"))
  (:Triggered
    (if (not (Variables|Default|GetIsInteractionLocked))
      (if (not (Variables|Default|GetIsPunching?))
        (Utilities|HandleDirectionInput (Utilities|Enum|LiteralenumE_RetroMovement "NewEnumerator3") "0.000000,-2.000000,1.000000" :!label _label)
        (Variables|Default|SetIsWalking? true))))
  (:Started
    (goto _label Started))
  (:Completed
    (Variables|Default|SetIsWalking? false)
    (goto _label Completed)))

(event Input|EnhancedActionEvents|EnhancedInputActionIA_Down
  (params (ActionValue :type Boolean) (ElapsedSeconds :type Float%20%28double-precision%29) (TriggeredSeconds :type Float%20%28double-precision%29) (InputAction :type Input%20Action%20Object%20Reference :default "/Game/Input/Actions/IA_Down.IA_Down"))
  (:Triggered
    (if (not (Variables|Default|GetIsInteractionLocked))
      (if (not (Variables|Default|GetIsPunching?))
        (Utilities|HandleDirectionInput (Utilities|Enum|LiteralenumE_RetroMovement "NewEnumerator2") "0.000000,-1.000000,0.000000" :!label _label)
        (Variables|Default|SetIsWalking? true))))
  (:Started
    (goto _label Started))
  (:Completed
    (Variables|Default|SetIsWalking? false)
    (goto _label Completed)))

(event Input|EnhancedActionEvents|EnhancedInputActionIA_Right
  (params (ActionValue :type Boolean) (ElapsedSeconds :type Float%20%28double-precision%29) (TriggeredSeconds :type Float%20%28double-precision%29) (InputAction :type Input%20Action%20Object%20Reference :default "/Game/Input/Actions/IA_Right.IA_Right"))
  (:Triggered
    (if (not (Variables|Default|GetIsInteractionLocked))
      (if (Variables|Default|GetIsPunching?)
        (Utilities|HandleDirectionInput (Utilities|Enum|LiteralenumE_RetroMovement "NewEnumerator0") "1.000000,0.000000,0.000000" :!label _label)
        (Variables|Default|SetIsWalking? true))))
  (:Started
    (goto _label Started))
  (:Completed
    (Variables|Default|SetIsWalking? false)
    (goto _label Completed)))

(event Collision|EventActorBeginOverlap
  (params (OtherActor :type Actor%20Object%20Reference))
  (|CallParentFunction OtherActor) ; This node is disabled and will not be called.\nDrag off pins to build functionality.
)

(event EventTick
  (params (DeltaSeconds :type Float%20%28single-precision%29))
  (|CallParentFunction DeltaSeconds) ; This node is disabled and will not be called.\nDrag off pins to build functionality.
)

(event Input|KeyboardEvents|SpaceBar
  (params (Key :type Key%20Structure))
  (bind _returnvalue (Game|GetPlayerController 0))
  (:Pressed
    (if (Variables|Default|GetFlySkillObtained?)
      _
      (else
        _))
    (Utilities|FlowControl|FlipFlop
      (:A
        (Pawn|Components|CharacterMovement|SetMovementMode (Variables|Character|GetCharacterMovement) "MOVE_Flying" 0)
        (Variables|Default|SetFlyActivated? true)
        (bind _flyup (Timeline|Move%20up Play)
          (:Update
            (Input|DisableInput _returnvalue)
            (Transformation|SetRelativeLocationAndRotation (Variables|Default|GetSprite) (Math|Vector|MakeVector 0.0 0.0 _flyup) "0, 0, 0" false false)
            (Utilities|FlowControl|DoOnce false
              (:Completed
                (Effects|SpawnEmitteratLocation "/Game/StarterContent/Particles/P_Explosion.P_Explosion" (Transformation|GetWorldLocation (Variables|Default|GetMoneyAbsorb))))))
          (:Finished
            (Input|EnableInput _returnvalue))))
      (:B
        (Pawn|Components|CharacterMovement|SetMovementMode (Variables|Character|GetCharacterMovement) "MOVE_Falling" 0)
        (Variables|Default|SetFlyActivated? false)))))

(fn ConstructionScript
  (|CallParentFunction))