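; BP_MainHuman is the main human character Blueprint, handling jump, landing and melee attack input with PaperZD-style animation overrides.
; A PlayerBehavior state gates jumps and punches, while override callbacks return it to Stand.
; Normal attacks cycle three animations through AttackCount, resetting after the third or a retriggerable delay, and a flag-gated BlockEat input plays another attack.
; PlayComboATK applies animation, damage and box-trace settings from ATKAnimData.
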(event Input|EnhancedActionEvents|EnhancedInputActionIA_BlockEat
  (params (ActionValue :type Boolean) (ElapsedSeconds :type Float%20%28double-precision%29) (TriggeredSeconds :type Float%20%28double-precision%29) (InputAction :type Input%20Action%20Object%20Reference :default "/Game/Input/Actions/IA_BlockEat.IA_BlockEat"))
  (:Started
    (if (not (Variables|Default|GetIsPunching?))
      (if (not (Variables|Default|GetIsWalking?))
        (if (not (Variables|Default|GetIsJumping?))
          (if (Variables|Default|GetATKWindowOpen)
            (Variables|Combat|SetComboActivated? true)
            (else
              (|PlayAnimationOverridewithCallbacks (Variables|/Script/PaperZD.PaperZDAnimationComponent|GetAnimInstance (Variables|Default|GetAnimationComponent)) "/Game/Character_BP+AS/Main_Human/AnimSequences/ATK3.ATK3" "DefaultSlot" 1.0 0.0))))))))

(event Input|EnhancedActionEvents|EnhancedInputActionIA_Jump
  (params (ActionValue :type Boolean) (ElapsedSeconds :type Float%20%28double-precision%29) (TriggeredSeconds :type Float%20%28double-precision%29) (InputAction :type Input%20Action%20Object%20Reference :default "/Game/Input/Actions/IA_Jump.IA_Jump"))
  (:Started
    (switch Utilities|FlowControl|Switch|SwitchonPlayerBehavior (Variables|Default|GetPlayerBehavior)
      (:NewEnumerator0
        _)
      (:NewEnumerator1
        _))
    (Character|Jump)
    (Variables|Default|SetIsJumping? true))
  (:Completed
    (Character|StopJumping)
    (Variables|Default|SetIsJumping? false)))

(event Input|EnhancedActionEvents|EnhancedInputActionIA_NormalATK
  (params (ActionValue :type Boolean) (ElapsedSeconds :type Float%20%28double-precision%29) (TriggeredSeconds :type Float%20%28double-precision%29) (InputAction :type Input%20Action%20Object%20Reference :default "/Game/Input/Actions/IA_NormalATK.IA_NormalATK"))
  ;[0 0 0] Punch
  (:Triggered
    (switch Utilities|FlowControl|Switch|SwitchonPlayerBehavior (Variables|Default|GetPlayerBehavior)
      (:NewEnumerator0
        (if (not (Variables|Default|GetIsPunching?))
          (Variables|Default|SetPlayerBehavior "NewEnumerator2")
          (|PlayAnimationOverridewithCallbacks (Class|PaperZDCharacter|GetAnimInstance) (Utilities|Select :Index (Variables|Combat|GetAttackCount) :Option%200 "/Game/Character_BP+AS/Main_Human/AnimSequences/ATK1.ATK1" :Option%201 "/Game/Character_BP+AS/Main_Human/AnimSequences/ComboATK1.ComboATK1" :Option%202 "/Game/Character_BP+AS/Main_Human/AnimSequences/ComboATK2.ComboATK2") "DefaultSlot" 1.0 0.0
            (:then
              (Variables|Default|SetIsPunching? true)
              (Math|Integer|IncrementInt (Variables|Combat|GetAttackCount)))
            (:OnCompleted
              (Variables|Default|SetIsPunching? false :!label _label)
              (Variables|Default|SetPlayerBehavior "NewEnumerator0")
              (if (== (Variables|Combat|GetAttackCount) 3)
                (Variables|Combat|SetAttackCount 0)
                (else
                  (Utilities|FlowControl|RetriggerableDelay 1.0)
                  (Variables|Combat|SetAttackCount 0))))
            (:OnCancelled
              (goto _label))))))))

(event EventOnLanded
  (params (Hit :type Hit%20Result%20Structure%20%28by%20ref%29))
  (Class|PaperZDAnimInstance|StopAllAnimationOverrides (Class|PaperZDCharacter|GetAnimInstance))
  (Variables|Default|SetPlayerBehavior "NewEnumerator5")
  (|PlayAnimationOverridewithCallbacks (Class|PaperZDCharacter|GetAnimInstance) "/Game/Character_BP+AS/Main_Human/AnimSequences/Land.Land" "DefaultSlot" 1.0 0.0
    (:OnCompleted
      _)
    (:OnCancelled
      _))
  (Variables|Default|SetPlayerBehavior "NewEnumerator0"))

(event Collision|EventActorBeginOverlap
  (params (OtherActor :type Actor%20Object%20Reference))
  (|CallParentFunction OtherActor) ; This node is disabled and will not be called.\nDrag off pins to build functionality.
)

(event EventTick
  (params (DeltaSeconds :type Float%20%28single-precision%29))
  (|CallParentFunction DeltaSeconds) ; This node is disabled and will not be called.\nDrag off pins to build functionality.
)

(event EventResetCombatVariables
  (CallFunction|SetEnableInput true)
  (Variables|Default|SetIsPunching? false)
  (Variables|Combat|SetComboActivated? false)
  (Variables|Default|SetATKWindowOpen false)
  (Variables|Combat|SetAttackCount 0)
  (Variables|Default|SetIsHopping? false)
  (Variables|Default|SetIsWalking? false)
  (Variables|Default|SetIsJumping? false))

(event EventBeginPlay
  (|CallParentFunction))

(fn ConstructionScript
  (|CallParentFunction))

(fn PlayComboATK
  (params (ATKCount :type Integer))
  (bind _atkanimdata (Variables|Combat|GetATKAnimData))
  (bind _output (Utilities|Array|Get(acopy) _atkanimdata ATKCount))
  (Class|PaperZDAnimInstance|PlayAnimationOverride (Variables|/Script/PaperZD.PaperZDAnimationComponent|GetAnimInstance (Variables|Default|GetAnimationComponent)) (.attackanimation _output) "DefaultSlot" 1.0 0.0)
  (Variables|Default|SetIn%20Damage (.attackdamage _output))
  (Variables|Default|SetTraceExtent (.boxtraceextent _output))
  (Transformation|SetRelativeLocation (Variables|Default|GetBoxTraceStart) (.boxtracestart _output) false false)
  (Transformation|SetRelativeLocation (Variables|Default|GetBoxTraceEnd) (.boxtraceend _output) false false))

(fn GetHitPlayHitReactAnimation
  (params (InDamage :type Float%20%28double-precision%29) (Instigator :type Actor%20Object%20Reference))
  (|CallParentFunction InDamage 0))