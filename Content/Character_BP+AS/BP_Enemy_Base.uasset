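; BP_Enemy_Base is a base enemy character with a health bar, AI state hooks, attack and death handling.
; A trigger overlap shows the health widget to nearby players, and health changes update its percentage.
; Events mirror combat target, alive, interacting and hit-reacting states into the AI Blackboard.
; Death clears the alive key, disables capsule collision and tick, hides the bar, and completes a quest task for the first player.
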(event OnComponentBeginOverlap(ShowHealth_Trigger)
  (params (OverlappedComponent :type Primitive%20Component%20Object%20Reference) (OtherActor :type Actor%20Object%20Reference) (OtherComp :type Primitive%20Component%20Object%20Reference) (OtherBodyIndex :type Integer) (bFromSweep :type Boolean) (SweepResult :type Hit%20Result%20Structure%20%28by%20ref%29))
  (bind _returnvalue (Game|GetInstigatorController OtherActor))
  ;[0 0 0] Show Health with Trigger Box, might need to set other condition in future.
  (Utilities|IsValid _returnvalue
    (:Is%20Valid
      (if (Class|Controller|IsPlayerController _returnvalue)
        (Development|SetHiddeninGame (Variables|Default|GetEnemyHealth_Widget) false false)))))

(event OnComponentEndOverlap(ShowHealth_Trigger)
  (params (OverlappedComponent :type Primitive%20Component%20Object%20Reference) (OtherActor :type Actor%20Object%20Reference) (OtherComp :type Primitive%20Component%20Object%20Reference) (OtherBodyIndex :type Integer))
  (bind _returnvalue (Game|GetInstigatorController OtherActor))
  ;[0 0 0] Show Health with Trigger Box, might need to set other condition in future.
  (Utilities|IsValid _returnvalue
    (:Is%20Valid
      (if (Class|Controller|IsPlayerController _returnvalue)
        (Development|SetHiddeninGame (Variables|Default|GetEnemyHealth_Widget) true false)))))

(event EventBeginPlay
  (|CallParentFunction)
  (Rendering|SetCastShadow (Variables|Default|GetEnemyHealth_Widget) false)
  (bind _aswbp_enemy_health_bar (Utilities|Casting|CastToWBP_EnemyHealthBar (UserInterface|GetUserWidgetObject (Variables|Default|GetEnemyHealth_Widget))))
  (Variables|Default|Set%20Enemy%20Health%20Bar _aswbp_enemy_health_bar)
  (AI|Components|Blackboard|SetValueasBool (AI|GetBlackboard (Pawn|GetController)) (Variables|Default|GetAlive%20BBkey) true)
  (AI|Components|Blackboard|SetValueasBool (AI|GetBlackboard (Pawn|GetController)) (Variables|Default|GetInteracting%20BBkey) true))

(event Collision|EventActorBeginOverlap
  (params (OtherActor :type Actor%20Object%20Reference))
  (|CallParentFunction OtherActor) ; This node is disabled and will not be called.\nDrag off pins to build functionality.
)

(event EventSetCombatTarget
  (params (CombatTarget :type Actor%20Object%20Reference))
  (AI|Components|Blackboard|SetValueasObject (AI|GetBlackboard (Pawn|GetController)) (Variables|Default|GetCombatTargetBBKeyName) CombatTarget))

(event EventAttack
  (params (TargetSide :type E_TargetSide%20Enum :default "NewEnumerator2"))
  (CallFunction|HitPlayAttackAnimation TargetSide)
  (Variables|Default|SetIn%20Damage 1e+01))

(event EventHandleDeath
  (params (DeathCauser :type Actor%20Object%20Reference))
  (CallFunction|Die)
  (CallFunction|CompleteQuestTask (Game|GetPlayerController 0) "NewEnumerator3" self))

(event EventSetHitReacting
  (params (IsHitReacting :type Boolean))
  (AI|Components|Blackboard|SetValueasBool (AI|GetBlackboard (Pawn|GetController)) (Variables|Default|GetHitReacting) IsHitReacting))

(event EventOnHealthChanged
  (params (CurrentHealth :type Float%20%28double-precision%29) (MaxHealth :type Float%20%28double-precision%29) (Instigator :type Actor%20Object%20Reference))
  (|CallParentFunction CurrentHealth MaxHealth Instigator)
  (Default|SetHealthPercent (Variables|Default|Get%20Enemy%20Health%20Bar) (Math|Float|SafeDivide CurrentHealth MaxHealth)))

(event EventInteractbool
  (params (IsInteracting :type Boolean))
  (Development|PrintString (Utilities|String|ToString(Boolean) IsInteracting))
  (AI|Components|Blackboard|SetValueasBool (AI|GetBlackboard (Pawn|GetController)) (Variables|Default|GetInteracting%20BBkey) IsInteracting))

(fn ConstructionScript
  (|CallParentFunction))

(fn GetHitPlayHitReactAnimation
  (params (InDamage :type Float%20%28double-precision%29) (Instigator :type Actor%20Object%20Reference))
  (|CallParentFunction InDamage 0))

(fn Die
  (Utilities|FlowControl|Sequence
    (:then_1
      ;[0 0 0] Disable Behavior Tree
      (AI|Components|Blackboard|SetValueasBool (AI|GetBlackboard (Pawn|GetController)) (Variables|Default|GetAlive%20BBkey) false))
    (:then_2
      ;[0 0 0] Disable Collision
      (Collision|SetCollisionEnabled (Variables|Default|GetCapsuleComponent) "NoCollision"))
    (:then_3
      ;[0 0 0] Hide Health Bar
      (Rendering|SetVisibility (Variables|Default|GetEnemyHealth_Widget) false false))
    (:then_4
      ;[0 0 0] Disable it
      (Actor|Tick|SetActorTickEnabled false))))

(fn GetHealth
  (return 0.0))