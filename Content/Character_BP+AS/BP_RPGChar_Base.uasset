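; Base sprite character for the RPG, providing shared melee combat, damage feedback and NPC-style dialogue.
; Attacks use directional animation overrides and a debug-drawn box trace that applies damage.
; Incoming damage updates BPCStats, then triggers particles, sound, red flash, time-dilation hit stop, conditional shake, floating numbers and hurt or death animations.
; Interaction locks the character and shows DataTable dialogue through the GameMode's HUD, chaining rows by NextRow.
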(event Custom|EnemyShake
  (bind _gethitlocation (Variables|Default|GetGethitLocation))
  ;[0 0 0] Make ATK Impactful
  (Variables|Default|SetGetHitLocation (Transformation|GetWorldLocation (Variables|Default|GetSprite)))
  (bind _newtrack_0 (Timeline|Timeline PlayFromStart)
    (:Update
      (Transformation|SetWorldLocation (Variables|Default|GetSprite) (Math|Vector|MakeVector (Math|Float|Lerp (- (.x _gethitlocation) 5.0) (+ (.x _gethitlocation) 5.0) _newtrack_0) (.y _gethitlocation) (.z _gethitlocation)) false false))))

(event Custom|FlashSprite%28TakeDmg%29
  ;[0 0 0] Make ATK Impactful
  (Sprite|SetSpriteColor (Variables|Default|GetSprite) "(R=1.000000,G=0.000000,B=0.058446,A=1.000000)")
  (Utilities|FlowControl|RetriggerableDelay (Variables|Combat|GetFlash%20Duration))
  (Sprite|SetSpriteColor (Variables|Default|GetSprite) "(R=1.000000,G=1.000000,B=1.000000,A=1.000000)"))

(event Custom|HitStop
  ;[0 0 0] Make ATK Impactful
  (Variables|Default|SetCustomTimeDilation 0.0)
  (Utilities|FlowControl|RetriggerableDelay 0.2)
  (Variables|Default|SetCustomTimeDilation 1.0))

(event EventBeginPlay
  (EventDispatchers|BindEventtoOnHealthChanged (Variables|Default|GetBPC_Stats) (EventDispatchers|CreateEvent :!event OnHealthChanged))
  (EventDispatchers|BindEventtoOnMaxHPStatisticChanged (Variables|Default|GetBPC_Stats) (EventDispatchers|CreateEvent :!event MaxHealthChanged))
  (Rendering|SetCastShadow (Variables|Default|GetDialogueIndicator) false)
  (Variables|Default|SetResetRowName (Variables|Default|GetCurrentRowName))
  (bind _asgm_rpg (Utilities|Casting|CastToGM_RPG (Game|GetGameMode)))
  (Variables|Default|SetGameMode _asgm_rpg))

(event Game|Damage|EventAnyDamage
  (params (Damage :type Float%20%28single-precision%29) (DamageType :type Damage%20Type%20Object%20Reference) (InstigatedBy :type Controller%20Object%20Reference) (DamageCauser :type Actor%20Object%20Reference))
  (CallFunction|GetHitPlayHitReactAnimation Damage DamageCauser))

(event EventFinishInteraction
  (CallFunction|EndInteraction)
  (Default|CallDialogueComplete))

(event EventInteractOLD
  (params (Instigator :type BP%20RPG%20Char%20Base%20Object%20Reference))
  (if (!= (Variables|Default|GetCurrentRowName) "")
    (CallFunction|StartInteraction Instigator)
    (CallFunction|StartInteraction Instigator)
    (bind _dialogue (CallFunction|ShowDialogueLine))
    (Development|PrintString _dialogue)))

(fn ConstructionScript
  (bind _boxtracestart (Variables|Default|GetBoxTraceStart))
  (bind _boxtraceend (Variables|Default|GetBoxTraceEnd))
  (bind _returnvalue (Transformation|GetWorldLocation _boxtraceend))
  (bind _returnvalue_2 (Transformation|GetWorldLocation _boxtracestart))
  (Class|KismetSystemLibrary|BoxTraceSingleforObjects _returnvalue_2 _returnvalue (Variables|Combat|GetTraceExtent) (Variables|Combat|GetBoxRotation) (Variables|Default|GetTraceObjectType) false 0 "ForDuration" true "(R=0.000000,G=1.000000,B=0.100263,A=1.000000)" "(R=1.000000,G=0.176427,B=0.000000,A=1.000000)" 1e+01)
  (Rendering|Debug|DrawDebugSphere _returnvalue_2 2e+01 12 "(R=0.061064,G=0.000000,B=1.000000,A=1.000000)" 5.0)
  (Rendering|Debug|DrawDebugSphere _returnvalue 2e+01 12 "(R=0.134885,G=0.000000,B=1.000000,A=1.000000)" 5.0))

(fn ShowDialogueLine
  (bind _returnvalue (Utilities|GetDataTableRow "/Game/DataTable/DT_HybridRPG_Dialogue.DT_HybridRPG_Dialogue" (Variables|Default|GetCurrentRowName))
    (:then
      (Default|ShowDialogue (Variables|/Game/Bluepints/GM_RPG.GM_RPG_C|GetHUDWidget (Variables|Default|GetGameMode)) self (Variables|Default|Get%20Name) (.DialogueText (Utilities|Struct|BreakS_DialogueData _returnvalue)))
      (Variables|Default|SetNext%20Row (.NextRow (Utilities|Struct|BreakS_DialogueData _returnvalue)))
      (return ""))))

(fn StartInteraction
  (params (InteractInstigator :type Actor%20Object%20Reference))
  (Variables|ActionLocked|SetIsInteractionLocked true)
  (Components|Movement|StopMovementImmediately (Variables|Character|GetCharacterMovement))
  (Audio|PlaySound2D 0 1.0 1.0 0.0 0 0))

(fn EndInteraction
  (Variables|ActionLocked|SetIsInteractionLocked false))

(fn UnlockandHideDialogue
  (CallFunction|EndInteraction)
  (Default|HideDialogue (Variables|/Game/Core/UI/Widgets/WBP_HUD.WBP_HUD_C|GetWBP_SpeechBubble (Variables|/Game/Bluepints/GM_RPG.GM_RPG_C|GetHUDWidget (Variables|Default|GetGameMode)))))

(fn ATKBoxTrace
  (bind _outhit (Class|KismetSystemLibrary|BoxTraceSingleforObjects (Transformation|GetWorldLocation (Variables|Default|GetBoxTraceStart)) (Transformation|GetWorldLocation (Variables|Default|GetBoxTraceEnd)) (Variables|Combat|GetTraceExtent) (Variables|Combat|GetBoxRotation) (Variables|Default|GetTraceObjectType) false 0 "ForDuration" true "(R=1.000000,G=0.000000,B=0.000000,A=1.000000)" "(R=0.000000,G=1.000000,B=0.000000,A=1.000000)" 1e+01))
  (Game|Damage|ApplyDamage (.HitActor (Collision|BreakHitResult _outhit)) (Variables|Combat|GetIn%20Damage) (Pawn|GetController) self))

(fn HitPlayAttackAnimation
  (params (TargetSide :type E_TargetSide%20Enum :default "NewEnumerator2"))
  (Class|PaperZDAnimInstance|PlayAnimationOverride (Variables|/Script/PaperZD.PaperZDAnimationComponent|GetAnimInstance (Variables|Default|GetAnimationComponent)) (Utilities|Select :Index TargetSide :NewEnumerator2 (Variables|Combat|GetAttackAnimSequenceLeft) :NewEnumerator3 (Variables|Combat|GetAttackAnimSequenceRight)) "DefaultSlot" 1.0 0.0))

(fn GetHitPlayHitReactAnimation
  (params (InDamage :type Float%20%28double-precision%29) (Instigator :type Actor%20Object%20Reference))
  (bind _output_get (Variables|Combat|SetIn%20Damage InDamage))
  (Utilities|FlowControl|Sequence
    (:then_0
      (Default|AddValuetoHealth (Variables|Default|GetBPC_Stats) (* _output_get -1.0) Instigator))
    (:then_1
      (CallFunction|SetEnableInput false))
    (:then_2
      (Niagara|SpawnSystematLocation (Variables|Combat|GetHitParticle) (Transformation|GetActorLocation)))
    (:then_3
      (Audio|PlaySound2D (Variables|Combat|GetGetHitSound) 1.0 1.0 0.0 0 0))
    (:then_4
      (CallFunction|FlashSprite(TakeDmg)))
    (:then_5
      (CallFunction|HitStop))
    (:then_6
      (CallFunction|CreateDamageNumberNotification (Variables|Combat|GetIn%20Damage) (Transformation|GetActorLocation)))
    (:then_7
      (CallFunction|PlayAnimBaseonHealth))
    (:then_8
      (if (Actor|ActorHasTag (Variables|Default|GetInstigator) "Enemy")
        (CallFunction|EnemyShake)))))

(fn PlayAnimBaseonHealth
  (if (<= (Variables|/Game/Components/BPC_Stats.BPC_Stats_C|GetCurrentHealth (Variables|Default|GetBPC_Stats)) 0.0)
    (bind _animationlength (Class|PaperZDAnimInstance|PlayAnimationOverride (Class|PaperZDCharacter|GetAnimInstance) (Variables|Combat|GetDeath%20Anim%20Sequence) "DefaultSlot" 1.0 0.0))
    (Variables|/Game/Components/BPC_Stats.BPC_Stats_C|SetIsDefeated? (Variables|Default|GetBPC_Stats) true)
    (if (Actor|ActorHasTag (Variables|Default|GetInstigator) "Player")
      (Class|PaperZDAnimInstance|StopAllAnimationOverrides (Variables|/Script/PaperZD.PaperZDAnimationComponent|GetAnimInstance (Variables|Default|GetAnimationComponent)))
      (Input|DisableInput 0)
      (else
        (Actor|SetLifeSpan (+ _animationlength 0.15))))
    (else
      (Class|PaperZDAnimInstance|PlayAnimationOverride (Variables|/Script/PaperZD.PaperZDAnimationComponent|GetAnimInstance (Variables|Default|GetAnimationComponent)) (Variables|Combat|GetHurt%20React%20Anim%20Sequence) "DefaultSlot" 1.0 0.0))))

(fn SetEnableInput
  (params (Enabled? :type Boolean))
  (bind _player_controller (Variables|Default|GetPlayer%20Controller))
  (Variables|Default|GetPlayer%20Controller
    (:then
      (if Enabled?
        (Input|EnableInput _player_controller)
        (else
          (Input|DisableInput _player_controller))))
    (:else)))

(fn CreateDamageNumberNotification
  (params (Number :type Float%20%28double-precision%29) (Location :type Vector))
  (Utilities|FlowControl|Sequence
    (:then_0
      ;[0 0 0] Create Number Widget
      (bind _returnvalue (UserInterface|CreateWidget "/Game/Core/UI/Widgets/WBP_DamageNumber.WBP_DamageNumber_C" (Game|GetPlayerController 0)))
      (bind _output_get (LocalVariables|SetNumberWidget _returnvalue))
      (UserInterface|Viewport|AddtoViewport _output_get 0))
    (:then_1
      ;[0 0 0] Set Number and Color
      (Default|SetNumber (LocalVariables|GetNumberWidget) Number (Variables|Combat|GetDamage%20Color%20and%20Opacity)))
    (:then_2
      ;[0 0 0] Set Position in Viewport
      (Class|UserWidget|SetPositioninViewport (LocalVariables|GetNumberWidget) (.ScreenPosition (Class|GameplayStatics|ProjectWorldtoScreen (Game|GetPlayerController 0) (Math|Vector|MakeVector (.x Location) (.y Location) (+ (.z Location) 75.0)) false)) true))
    (:then_3
      ;[0 0 0] Play Number Floationg Animation
      (UserInterface|Animation|PlayAnimation (LocalVariables|GetNumberWidget) (Variables|/Game/Core/UI/Widgets/WBP_DamageNumber.WBP_DamageNumber_C|GetFloatAnimation (LocalVariables|GetNumberWidget)) 0.0 1 "Forward" 1.0 false))))

(fn AddTrackArrow
  (params (Location :type Vector))
  (Variables|Default|GetTrackArrow
    (:then)
    (:else
      (bind _returnvalue (Game|SpawnActorfromClass "/Game/Quest/BP_TrackArrow.BP_TrackArrow_C" (Transformation|GetWorldTransform (Variables|Default|GetSprite)) "AlwaysSpawn" "MultiplyWithRoot" 0 0))
      (bind _output_get (Variables|Default|SetTrackArrow _returnvalue))
      (Transformation|AttachComponentToComponent _output_get (Variables|Default|GetSprite) "None" "SnapToTarget" "KeepRelative" "SnapToTarget" true))))

(fn OnHealthChanged
  (params (CurrentHealth :type Float%20%28double-precision%29) (MaxHealth :type Float%20%28double-precision%29) (Instigator :type Actor%20Object%20Reference))
  (if (<= CurrentHealth 0.0)
    (CallFunction|HandleDeath Instigator)))

(fn HandleDeath
  (params (DeathCauser :type Actor%20Object%20Reference)))

(fn MaxHealthChanged
  (params (CurrentHealth :type Float%20%28double-precision%29) (CurrentMAXHealth :type Float%20%28double-precision%29) (Max+Equipment%20Health :type Float%20%28double-precision%29) (EquipmentHealth :type Float%20%28double-precision%29)))

(fn GetBubbleLocation
  (return (Transformation|GetWorldLocation (Variables|Default|GetDialogueIndicator))))

(fn ShowNextLine
  (if (Utilities|Array|IsEmpty (Variables|Default|GetNext%20Row))
    (Variables|Default|SetCurrentRowName (Variables|Default|GetResetRowName))
    (return false false)
    (else
      (Variables|Default|SetCurrentRowName (Utilities|String|StringToName (Variables|Default|GetNext%20Row)))
      (CallFunction|ShowDialogueLine)
      (Audio|PlaySound2D 0 1.0 1.0 0.0 0 0)
      (return true false))))