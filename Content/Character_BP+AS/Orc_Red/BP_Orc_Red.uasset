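; BP_Orc_Red is a red orc character, a child Blueprint that overrides the parent's Play Anim Base on Health to pick directional hurt and death animations.
; After the parent call, it checks BPCStats health and plays an animation override through the AnimationComponent's AnimInstance.
; While alive, the hurt variant follows the player's X position relative to BoxTraceStart.
; At zero health, the death variant follows the orc's facing along X.
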(event Collision|EventActorBeginOverlap
  (params (OtherActor :type Actor%20Object%20Reference))
  (|CallParentFunction OtherActor) ; This node is disabled and will not be called.\nDrag off pins to build functionality.
)

(fn ConstructionScript
  (|CallParentFunction))

(fn PlayAnimBaseonHealth
  (|CallParentFunction)
  (if (> (Variables|/Game/Components/BPC_Stats.BPC_Stats_C|GetCurrentHealth (Variables|Default|GetBPC_Stats)) 0.0)
    (if (> (.X (Math|Vector|BreakVector (- (Transformation|GetWorldLocation (Variables|Default|GetBoxTraceStart)) (Transformation|GetActorLocation (Game|GetPlayerCharacter 0))))) 0.0)
      (Class|PaperZDAnimInstance|PlayAnimationOverride (Variables|/Script/PaperZD.PaperZDAnimationComponent|GetAnimInstance (Variables|Default|GetAnimationComponent)) "/Game/Character_BP+AS/Orc_Red/AnimSequences/HurtL.HurtL" "DefaultSlot" 1.0 0.0)
      (else
        (Class|PaperZDAnimInstance|PlayAnimationOverride (Variables|/Script/PaperZD.PaperZDAnimationComponent|GetAnimInstance (Variables|Default|GetAnimationComponent)) (Variables|Default|GetHurt%20React%20Anim%20Sequence) "DefaultSlot" 1.0 0.0)))
    (elif (> (.X (Math|Vector|BreakVector (Math|Rotator|GetRotationXVector (Transformation|GetActorRotation)))) 0.0)
      (Class|PaperZDAnimInstance|PlayAnimationOverride (Variables|/Script/PaperZD.PaperZDAnimationComponent|GetAnimInstance (Variables|Default|GetAnimationComponent)) (Variables|Default|GetDeath%20Anim%20Sequence) "DefaultSlot" 1.0 0.0)
      (else
        (Class|PaperZDAnimInstance|PlayAnimationOverride (Variables|/Script/PaperZD.PaperZDAnimationComponent|GetAnimInstance (Variables|Default|GetAnimationComponent)) "/Game/Character_BP+AS/Orc_Red/AnimSequences/DeadL.DeadL" "DefaultSlot" 1.0 0.0)))))