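; BP_VFX is a visual effect actor that shows a Paper2D flipbook and then removes itself.
; On BeginPlay it assigns its flipbook variable to the sprite component and starts a timer set to the flipbook's frame count divided by three, in seconds.
; When the timer fires, the actor destroys itself and clears the timer handle.
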(event Custom|Destroy%20actor
  (Actor|DestroyActor)
  (Utilities|Time|ClearandInvalidateTimerbyHandle (Variables|Default|GetPlay%20Rate%20Timer)))

(event EventBeginPlay
  (Sprite|SetFlipbook (Variables|Default|GetSprite) (Variables|Default|GetNew%20Flipbook))
  (bind _returnvalue (Utilities|Time|SetTimerbyEvent (delegate Custom|Destroy%20actor) (Math|Conversions|ToFloat(Integer) (/ (Class|PaperFlipbookComponent|GetFlipbookLengthinFrames (Variables|Default|GetSprite)) 3))))
  (Variables|Default|SetPlay%20Rate%20Timer _returnvalue))

(fn ConstructionScript)