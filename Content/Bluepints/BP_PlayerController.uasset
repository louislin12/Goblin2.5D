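; Player controller that manages character transformation, the RPG HUD and coin and crystal totals.
; Holding X shows the transform widget, while BeginPlay builds the stat HUD and starts as Goblin.
; PosessBlueprint saves health to the game instance, spawns the DT_TransformPower character in place, possesses it and destroys the old one, with a lock released shortly after switching.
; Transformation adds per-form sounds, icons and effects; debug keys test health and level loading.
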(event Custom|OnCharacterSwitch
  (Utilities|FlowControl|Delay 0.2)
  (Variables|Default|SetLockPossess false))

(event Custom|Add%20Crystals
  (params (Crystals%20to%20Add :type S%20Money%20Structure))
  (bind (_name _amount _paperflipbook _crystal_) (Utilities|Struct|BreakS_Money Crystals%20to%20Add))
  ;[0 0 0] Add crystals and coins
  (if _crystal_
    (Variables|Default|SetTotal%20Crystal (+ _amount (Variables|Default|GetTotal%20Crystal)))))

(event Custom|Add%20Coin
  (params (Coins%20to%20Add :type S%20Money%20Structure))
  (bind (_name _amount _paperflipbook _crystal_) (Utilities|Struct|BreakS_Money Coins%20to%20Add))
  ;[0 0 0] Add crystals and coins
  (if (not _crystal_)
    (Variables|Default|SetTotal%20Coins (+ _amount (Variables|Default|GetTotal%20Coins)))))

(event EventBeginPlay
  ;[0 0 0] HP HUD
  (bind _returnvalue (UserInterface|CreateWidget "/Game/Widgets/WBP_RPGHUD.WBP_RPGHUD_C" (Game|GetPlayerController 0)))
  (bind _output_get (Variables|Default|SetWBP%20Hud%20Overlay _returnvalue))
  (UserInterface|Viewport|AddtoViewport _output_get 0)
  (CallFunction|HUDSetup _output_get)
  (EventDispatchers|BindEventtoCharacterSwitch (delegate Custom|OnCharacterSwitch))
  (CallFunction|PosessBlueprint "Goblin"))

(event EventTick
  (params (DeltaSeconds :type Float%20%28single-precision%29)))

(event EventUpdateHealthWidget
  (params (CurrentHealth :type Float%20%28double-precision%29) (MaxHealth :type Float%20%28double-precision%29))
  (bind _wbp_hud_overlay (Variables|Default|GetWBP%20Hud%20Overlay))
  (Utilities|IsValid _wbp_hud_overlay
    (:Is%20Valid
      (Default|UpdateHealthWidget (Variables|/Game/Widgets/WBP_RPGHUD.WBP_RPGHUD_C|GetWBP_PlayerHealthBar _wbp_hud_overlay) CurrentHealth MaxHealth))))

(event Input|KeyboardEvents|DebugKeyNumPadNine
  (params (Key :type Key%20Structure :default "None") (ActionValue :type Input%20Action%20Value%20Structure))
  (:Pressed
    (Game|OpenLevel(byObjectReference) "/Game/Level/000_DevelopmentLevel.000_DevelopmentLevel")))

(event Input|KeyboardEvents|DebugKeySubtract
  (params (Key :type Key%20Structure :default "None") (ActionValue :type Input%20Action%20Value%20Structure))
  (:Pressed
    (Default|GetHitPlayHitReactAnimation (Variables|Default|GetMain%20Character) 1e+01)))

(event Input|KeyboardEvents|DebugKeyAdd
  (params (Key :type Key%20Structure :default "None") (ActionValue :type Input%20Action%20Value%20Structure))
  (:Pressed
    (Default|AddValuetoHealth (Variables|Default|GetBPC_Stats) 1e+01)))

(event Input|KeyboardEvents|X
  (params (Key :type Key%20Structure :default "None"))
  (bind _returnvalue (Game|GetPlayerController 0))
  ;[0 0 0] Press X for Switch
  (:Pressed
    (bind _returnvalue_2 (UserInterface|CreateWidget "/Game/Widgets/WBP_Transform.WBP_Transform_C"))
    (bind _output_get (Variables|Default|SetWBP_Transform _returnvalue_2))
    (UserInterface|Viewport|AddtoViewport _returnvalue_2 0)
    (Input|SetInputModeGameandUI _returnvalue 0 "DoNotLock" true false)
    (Variables|/Script/Engine.PlayerController|SetbShowMouseCursor _returnvalue true))
  (:Released
    (Widget|RemovefromParent _returnvalue_2)
    (Input|SetInputModeGameOnly _returnvalue false)
    (Variables|/Script/Engine.PlayerController|SetbShowMouseCursor _returnvalue false)))

(fn ConstructionScript)

(fn Transformation
  (bind _returnvalue (Game|GetPlayerCharacter 0))
  (bind _capsulecomponent (Variables|/Script/Engine.Character|GetCapsuleComponent _returnvalue))
  (bind _returnvalue_2 (Transformation|GetWorldLocation _capsulecomponent))
  (bind _output_get (Variables|Default|SetE_Transformation (Utilities|Array|Get(acopy) (Variables|Default|GetE_TransformIndex) (Variables|Default|GetCurrent%20Transformation))))
  (switch Utilities|FlowControl|Switch|SwitchonE_TransformPower _output_get
    (:NewEnumerator0
      (CallFunction|PosessBlueprint (Utilities|String|StringToName (Utilities|String|EnumtoString (Variables|Default|GetE_Transformation))) "/Game/Sound/MainGoblin/触碰-可爱声效_Cue.触碰-可爱声效_Cue")
      (CallFunction|SetupEXPIcon (Utilities|String|StringToName (Utilities|String|EnumtoString (Variables|Default|GetE_Transformation)))))
    (:NewEnumerator1
      (CallFunction|PosessBlueprint (Utilities|String|StringToName (Utilities|String|EnumtoString (Variables|Default|GetE_Transformation))) "/Game/Sound/MainOrc/Orc_Sound_Cue.Orc_Sound_Cue")
      (CallFunction|SetupEXPIcon (Utilities|String|StringToName (Utilities|String|EnumtoString (Variables|Default|GetE_Transformation)))))
    (:NewEnumerator2
      (CallFunction|PosessBlueprint (Utilities|String|StringToName (Utilities|String|EnumtoString (Variables|Default|GetE_Transformation)))))
    (:NewEnumerator3
      (CallFunction|PosessBlueprint (Utilities|String|StringToName (Utilities|String|EnumtoString (Variables|Default|GetE_Transformation)))))
    (:NewEnumerator4
      (CallFunction|PosessBlueprint (Utilities|String|StringToName (Utilities|String|EnumtoString (Variables|Default|GetE_Transformation))))
      (CallFunction|SetupEXPIcon (Utilities|String|StringToName (Utilities|String|EnumtoString (Variables|Default|GetE_Transformation)))))
    (:NewEnumerator5
      (CallFunction|PosessBlueprint (Utilities|String|StringToName (Utilities|String|EnumtoString (Variables|Default|GetE_Transformation))) "/Game/Sound/MainDragon/dragon-hurt-47161.dragon-hurt-47161")
      (CallFunction|SetupEXPIcon (Utilities|String|StringToName (Utilities|String|EnumtoString (Variables|Default|GetE_Transformation))))
      (Niagara|SpawnSystematLocation "/Game/Niagara/NS_StylizedFire.NS_StylizedFire" (- _returnvalue_2 "0.000000,50.000000,50.000000")))
    (:NewEnumerator6
      (CallFunction|PosessBlueprint (Utilities|String|StringToName (Utilities|String|EnumtoString (Variables|Default|GetE_Transformation))) "/Game/StarterContent/Audio/Explosion_Cue.Explosion_Cue")
      (CallFunction|SetupEXPIcon (Utilities|String|StringToName (Utilities|String|EnumtoString (Variables|Default|GetE_Transformation))))
      (Effects|SpawnEmitteratLocation "/Game/StarterContent/Particles/P_Explosion.P_Explosion" _returnvalue_2))))

(fn PosessBlueprint
  (params (RowName :type Name) (Sound :type Sound%20Base%20Object%20Reference))
  (if (not (Variables|Default|GetLockPossess))
    (Variables|Default|SetLockPossess true)
    (Variables|Default|SetOldCharacter (Game|GetPlayerCharacter 0))
    (bind _charactertype (Class|BPICharacterInterace|GetCharacterType(Message) (Variables|Default|GetOldCharacter)))
    (bind _currenthealth (Class|BPICharacterInterace|GetHealth(Message) (Variables|Default|GetOldCharacter)))
    (Class|BPIGameInstance|SaveCharacterHealth(Message) (Game|GetGameInstance) _charactertype _currenthealth)
    (Audio|PlaySound2D Sound 1.0 1.0 0.0 0 0)
    (bind _returnvalue (Utilities|GetDataTableRow "/Game/DataTable/DT_TransformPower.DT_TransformPower" RowName)
      (:then
        (bind _returnvalue_2 (Game|SpawnActorfromClass (.CharacterBlueprints (Utilities|Struct|BreakS_TransformationDescription _returnvalue)) (Transformation|GetWorldTransform (Variables|/Script/Engine.Character|GetCapsuleComponent (Game|GetPlayerCharacter 0))) "AlwaysSpawn" "MultiplyWithRoot" 0 0))
        (Pawn|Possess (Game|GetPlayerController 0) _returnvalue_2)
        (Utilities|IsValid (Variables|Default|GetOldCharacter)
          (:Is%20Valid
            (Actor|DestroyActor (Variables|Default|GetOldCharacter)))
          (:Is%20Not%20Valid
            _))
        (Default|CallCharacterSwitch)))))

(fn HUDSetup
  (params (self2 :type WBP%20RPGHUD%20Object%20Reference))
  (bind _wbp_hud_overlay (Variables|Default|GetWBP%20Hud%20Overlay))
  (bind _bpc_stats (Variables|Default|GetBPC_Stats))
  (bind _bpc_stats_2 (Variables|Default|GetBPC_Stats))
  (bind _bpc_stats_3 (Variables|Default|GetBPC_Stats))
  (bind _wbp_playerhealthbar (Variables|/Game/Widgets/WBP_RPGHUD.WBP_RPGHUD_C|GetWBP_PlayerHealthBar self2))
  (bind _currenthealth (Variables|/Game/Components/BPC_Stats.BPC_Stats_C|GetCurrentHealth _bpc_stats_3))
  (bind _maxhealth (Variables|/Game/Components/BPC_Stats.BPC_Stats_C|GetMaxHealth _bpc_stats_3))
  (bind _current_stamina (Variables|/Game/Components/BPC_Stats.BPC_Stats_C|GetCurrent%20Stamina _bpc_stats))
  (bind _maxstamina (Variables|/Game/Components/BPC_Stats.BPC_Stats_C|GetMaxStamina _bpc_stats))
  (bind _wbp_playestaminabar (Variables|/Game/Widgets/WBP_RPGHUD.WBP_RPGHUD_C|GetWBP_PlayeStaminaBar _wbp_hud_overlay))
  ;[0 0 0] HP FROM BPCHEALTH
  (Variables|/Script/UMG.ProgressBar|SetPercent (Variables|/Game/Widgets/WBP_PlayerHealthBar.WBP_PlayerHealthBar_C|GetProgressBarHealth _wbp_playerhealthbar) (/ _currenthealth _maxhealth))
  (Variables|/Script/UMG.TextBlock|SetText (Variables|/Game/Widgets/WBP_PlayerHealthBar.WBP_PlayerHealthBar_C|GetTextBlock_Health _wbp_playerhealthbar) (Utilities|Text|ToText(Float) _currenthealth "HalfToEven"))
  (Variables|/Script/UMG.TextBlock|SetText (Variables|/Game/Widgets/WBP_PlayerHealthBar.WBP_PlayerHealthBar_C|GetTextBlock_MaxHealth _wbp_playerhealthbar) (Utilities|Text|ToText(Float) _maxhealth "HalfToEven"))
  ;[0 0 0] Stamina from BPCHEALTH
  (Variables|/Script/UMG.ProgressBar|SetPercent (Variables|/Game/Widgets/WBP_PlayeStaminaBar.WBP_PlayeStaminaBar_C|GetProgressBarStamina _wbp_playestaminabar) (/ _current_stamina _maxstamina))
  (Variables|/Script/UMG.TextBlock|SetText (Variables|/Game/Widgets/WBP_PlayeStaminaBar.WBP_PlayeStaminaBar_C|GetTextBlock_Stamina _wbp_playestaminabar) (Utilities|Text|ToText(Float) _current_stamina "HalfToEven"))
  (Variables|/Script/UMG.TextBlock|SetText (Variables|/Game/Widgets/WBP_PlayeStaminaBar.WBP_PlayeStaminaBar_C|GetTextBlock_MaxStamina _wbp_playestaminabar) (Utilities|Text|ToText(Float) _maxstamina "HalfToEven"))
  (Variables|/Game/Widgets/WBP_EXP.WBP_EXP_C|SetPercent (Variables|/Game/Widgets/WBP_RPGHUD.WBP_RPGHUD_C|GetWBP_EXP (Variables|Default|GetWBP%20Hud%20Overlay)) (/ (Variables|/Game/Components/BPC_Stats.BPC_Stats_C|GetMana _bpc_stats_2) (Variables|/Game/Components/BPC_Stats.BPC_Stats_C|GetMaxMana _bpc_stats_2))))

(fn SetupEXPIcon
  (params (RowName :type Name))
  (bind _returnvalue (Utilities|GetDataTableRow "/Game/DataTable/DT_TransformPower.DT_TransformPower" RowName)
    (:then
      (Class|Image|SetBrush (Variables|/Game/Widgets/WBP_EXP.WBP_EXP_C|GetMainCharacterImage (Variables|/Game/Widgets/WBP_RPGHUD.WBP_RPGHUD_C|GetWBP_EXP (Variables|Default|GetWBP%20Hud%20Overlay))) (Class|PaperSpriteBlueprintLibrary|MakeBrushfromSprite (.Thumbnail (Utilities|Struct|BreakS_TransformationDescription _returnvalue)))))))

(fn GetCharacterType
  (return "NewEnumerator0"))

(fn GetHealth
  (return 0.0))